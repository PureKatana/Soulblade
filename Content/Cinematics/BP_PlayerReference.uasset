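; Cinematic proxy for the player, exposing events that cutscenes can use to control the live player character and controller.
; Each event fetches player zero's character or controller by cast and forwards the call, holding almost no logic itself.
; Events toggle input and UI together, set the first soul fragment cutscene flag, adjust mesh glow, move the character to a location and play a soul-pickup montage.
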(event `DisablePlayerInputAndUI`
  (bind _returnvalue (`GameplayStatics.GetPlayerController` 0))
  (bind _asbp_player_controller (cast `/Game/GKnight/BP_PlayerController` _returnvalue))
  (`self.DisableInput` (cast `/Game/GKnight/BP_PlayerCharacter` (`GameplayStatics.GetPlayerCharacter` 0) :!pure true) _returnvalue)
  (`/Game/GKnight/BP_PlayerController.DisableUI` _asbp_player_controller))

(event `EnablePlayerInputAndUI`
  (bind _asbp_player_controller (cast `/Game/GKnight/BP_PlayerController` (`GameplayStatics.GetPlayerController` 0)))
  (`self.EnableInput` (cast `/Game/GKnight/BP_PlayerCharacter` (`GameplayStatics.GetPlayerCharacter` 0) :!pure true) _asbp_player_controller)
  (`/Game/GKnight/BP_PlayerController.EnableUI` _asbp_player_controller))

(event `SetStartCutscene`
  (params (`bCanTakeFirstSoul?` :type Boolean))
  (bind _asbp_player_character (cast `/Game/GKnight/BP_PlayerCharacter` (`GameplayStatics.GetPlayerCharacter` 0)))
  (`/Game/GKnight/BP_PlayerCharacter.SetStartFirstSoulFragmentCutscene` _asbp_player_character `bCanTakeFirstSoul?`))

(event `SetCharacterMeshGlow`
  (params (IntensityValue :type "Float (single-precision)") (PowerValue :type "Float (single-precision)"))
  (bind _asbp_player_character (cast `/Game/GKnight/BP_PlayerCharacter` (`GameplayStatics.GetPlayerCharacter` 0)))
  (`/Game/GKnight/BP_PlayerCharacter.SetCharacterMeshGlow` _asbp_player_character IntensityValue PowerValue))

(event `MoveTo`
  (params (LocationToMove :type "Vector Structure"))
  (set `self.LocationToMove` LocationToMove)
  (bind _asbp_player_character (cast `/Game/GKnight/BP_PlayerCharacter` (`GameplayStatics.GetPlayerCharacter` 0)))
  (`/Game/GKnight/BP_PlayerCharacter.MoveToLocationCutscene` _asbp_player_character (`self.LocationToMove`)))

(event `PlayGetSoulAnim`
  (bind _asbp_player_character (cast `/Game/GKnight/BP_PlayerCharacter` (`GameplayStatics.GetPlayerCharacter` 0)))
  (`|PlayMontage` (`Character.Mesh` _asbp_player_character) "/Game/GKnight/Animation/GetSoul/Standing_Taunt_Battlecry__4__Montage.Standing_Taunt_Battlecry__4__Montage"))

(fn `UserConstructionScript`)