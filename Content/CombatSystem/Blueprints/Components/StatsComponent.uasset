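; Combat system component that holds an actor's stats as base/max and current value maps, initializing current values from base.
; Changes clamp between zero and max, broadcast an update event, and can request regeneration.
; Only Stamina regenerates, via a retriggerable delay before a looping timer that runs until full.
; TakeDamage lowers Health and sets the owner's StateManagerComponent to Dead at zero.
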(event `StartRegen`
  (params (`Stat Type` :type "/Game/CombatSystem/Blueprints/Enums/E_Stats Enum" :default "NewEnumerator0"))
  (switch `/Game/CombatSystem/Blueprints/Enums/E_Stats` `Stat Type`
    (:`NewEnumerator2`
      (`KismetSystemLibrary.K2_ClearTimer` null "RegenStamina")
      (`KismetSystemLibrary.RetriggerableDelay` 1.5)
      (`KismetSystemLibrary.K2_SetTimer` null "RegenStamina" 0.05 true))))

(fn `GetBaseStatsValue`
  (params (Stats :type "/Game/CombatSystem/Blueprints/Enums/E_Stats Enum" :default "NewEnumerator0"))
  (returns (`Base Value` :type "Float (double-precision)"))
  (return (break `/Game/CombatSystem/Blueprints/Structs/F_BaseStat` (`BlueprintMapLibrary.Map_Find` (`self.BaseStats`) Stats))))

(fn `GetCurrentStatValue`
  (params (Stats :type "/Game/CombatSystem/Blueprints/Enums/E_Stats Enum" :default "NewEnumerator0"))
  (returns (Value :type "Float (double-precision)"))
  (return (`BlueprintMapLibrary.Map_Find` (`self.CurrentStats`) Stats)))

(fn `GetMaxStatsValue`
  (params (Stats :type "/Game/CombatSystem/Blueprints/Enums/E_Stats Enum" :default "NewEnumerator0"))
  (returns (`Max Value` :type "Float (double-precision)"))
  (return (`.MaxValue_4_04E60A034FE99A155757138FFD8DDB8A` (break `/Game/CombatSystem/Blueprints/Structs/F_BaseStat` (`BlueprintMapLibrary.Map_Find` (`self.BaseStats`) Stats)))))

(fn `InitializeStats`
  (bind _keys (`BlueprintMapLibrary.Map_Keys` (`self.BaseStats`)))
  (for _array_element _keys
    (`self.SetCurrentStatValue` _array_element (break `/Game/CombatSystem/Blueprints/Structs/F_BaseStat` (`BlueprintMapLibrary.Map_Find` (`self.BaseStats`) _array_element)))))

(fn `ModifyCurrentStatValue`
  (params (Stats :type "/Game/CombatSystem/Blueprints/Enums/E_Stats Enum" :default "NewEnumerator0") (Value :type "Float (double-precision)") (`bShouldRegenerate?` :type Boolean :default true))
  (locals (L_Value :type "Float (double-precision)"))
  (if (!= Value 0.0)
    (bind _output_get (set `local.L_Value` (+ (`self.GetCurrentStatValue` (`local.Stats`)) (`local.Value`))))
    (bind _output_get_2 (set `local.L_Value` (`KismetMathLibrary.FClamp` _output_get 0.0 (`self.GetMaxStatsValue` (`local.Stats`)))))
    (`self.SetCurrentStatValue` (`local.Stats`) _output_get_2)
    (if (`local.bShouldRegenerate?`)
      (`self.StartRegen` (`local.Stats`)))))

(fn `RegenStamina`
  (`self.SetCurrentStatValue` "NewEnumerator2" (`KismetMathLibrary.FClamp` (+ (`self.GetCurrentStatValue` "NewEnumerator2") (`self.StaminaRegeneration`)) 0.0 (`self.GetMaxStatsValue` "NewEnumerator2")))
  (if (>= (`self.GetCurrentStatValue` "NewEnumerator2") (`self.GetMaxStatsValue` "NewEnumerator2"))
    (`KismetSystemLibrary.K2_ClearTimer` null "RegenStamina")))

(fn `SetBaseStatValue`
  (params (Stats :type "/Game/CombatSystem/Blueprints/Enums/E_Stats Enum" :default "NewEnumerator0") (Value :type "Float (double-precision)"))
  (bind _structout (setmembers `/Game/CombatSystem/Blueprints/Structs/F_BaseStat` :`StructRef` (`BlueprintMapLibrary.Map_Find` (`self.BaseStats`) Stats) :`BaseValue` Value))
  (`BlueprintMapLibrary.Map_Add` (`self.BaseStats`) (`local.Stats`) _structout))

(fn `SetCurrentStatValue`
  (params (Stats :type "/Game/CombatSystem/Blueprints/Enums/E_Stats Enum" :default "NewEnumerator0") (Value :type "Float (double-precision)"))
  (`BlueprintMapLibrary.Map_Add` (`self.CurrentStats`) Stats Value)
  (`self.OnCurrentStatValueUpdated` (`local.Stats`) (`local.Value`)))

(fn `SetMaxStatValue`
  (params (Stats :type "/Game/CombatSystem/Blueprints/Enums/E_Stats Enum" :default "NewEnumerator0") (Value :type "Float (double-precision)"))
  (bind _structout (setmembers `/Game/CombatSystem/Blueprints/Structs/F_BaseStat` :`StructRef` (`BlueprintMapLibrary.Map_Find` (`self.BaseStats`) Stats) :`MaxValue` Value))
  (`BlueprintMapLibrary.Map_Add` (`self.BaseStats`) (`local.Stats`) _structout))

(fn `TakeDamage`
  (params (Damage :type "Float (double-precision)"))
  (`self.ModifyCurrentStatValue` "NewEnumerator1" (* (`local.Damage`) -1.0))
  (if (<= (`self.GetCurrentStatValue` "NewEnumerator1") 0.0)
    (`/Game/CombatSystem/Blueprints/Components/StateManagerComponent.SetState` (`Actor.GetComponentByClass` (`self.GetOwner`) "/Game/CombatSystem/Blueprints/Components/StateManagerComponent.StateManagerComponent_C") (struct :`TagName` "Character.State.Dead"))))