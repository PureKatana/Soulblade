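; CollisionComponent is a combat component that detects hits by sweeping a sphere trace between two sockets on an assigned mesh.
; While collision is enabled, Tick runs a multi-sphere object trace that respects an ignore list.
; Each newly hit actor is recorded and reported once through the OnHit dispatcher.
; Enabling collision clears the hit list, so each activation window can hit an actor again.
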(event `self.ReceiveTick`
  (params (DeltaSeconds :type "Float (single-precision)"))
  (if (`self.bIsCollisionEnabled?`)
    (`self.CollisionTrace`)))

(event `CollisionTrace`
  (bind _collisionmeshcomponent (`self.CollisionMeshComponent`))
  ;[1 1 1] Collision Trace
  (bind _outhits (`KismetSystemLibrary.SphereTraceMultiForObjects` (`SceneComponent.GetSocketLocation` _collisionmeshcomponent (`self.Start Socket Name`)) (`SceneComponent.GetSocketLocation` _collisionmeshcomponent (`self.End Socket Name`)) (`self.TraceRadius`) (`self.Collision Object Types`) false (`self.Actors to Ignore`) (`self.Draw Debug Type`)))
  (for _array_element _outhits
    (bind _output_get (set `self.Last Hit` _array_element))
    (bind (_bblockinghit _binitialoverlap _time _distance _location _impactpoint _normal _impactnormal _physmat _hitactor) (`GameplayStatics.BreakHitResult` _output_get))
    (if (not (`KismetArrayLibrary.Array_Contains` (`self.AlreadyHitActors`) _hitactor))
      (bind _output_get_2 (set `self.Hit Actor` _hitactor))
      (`KismetArrayLibrary.Array_Add` (`self.AlreadyHitActors`) _output_get_2)
      (`self.OnHit` (`self.Last Hit`)))))

(event `EnableCollision`
  (`self.ClearHitActors`)
  (set `self.bIsCollisionEnabled?` true))

(event `DisableCollision`
  (set `self.bIsCollisionEnabled?` false))

(event `ClearHitActors`
  (`KismetArrayLibrary.Array_Clear` (`self.AlreadyHitActors`)))

(fn `AddActorToIgnore`
  (params (ActorToAdd :type "Actor Object Reference (by ref)"))
  (`KismetArrayLibrary.Array_AddUnique` (`self.Actors to Ignore`) ActorToAdd))

(fn `GetActorsToIgnore`
  (returns (`Return Value` :type "Array of Actor Object Reference"))
  (return (`self.Actors to Ignore`)))

(fn `GetAlreadyHitActors`
  (returns (`Return Value` :type "Array of Actor Object Reference"))
  (return (`self.AlreadyHitActors`)))

(fn `GetCollisionMeshComponent`
  (returns (`Return Value` :type "PrimitiveComponent Object Reference"))
  (return (`self.CollisionMeshComponent`)))

(fn `GetLastHit`
  (returns (`Return Value` :type "HitResult Structure"))
  (return (`self.Last Hit`)))

(fn `IsCollisionEnabled?`
  (returns (`Return Value` :type Boolean))
  (return (`self.bIsCollisionEnabled?`)))

(fn `RemoveActorToIgnore`
  (params (ActorToRemove :type "Actor Object Reference (by ref)"))
  (`KismetArrayLibrary.Array_RemoveItem` (`self.Actors to Ignore`) ActorToRemove))

(fn `SetCollisionMeshComponent`
  (params (MeshComponent :type "PrimitiveComponent Object Reference"))
  (set `self.CollisionMeshComponent` MeshComponent))