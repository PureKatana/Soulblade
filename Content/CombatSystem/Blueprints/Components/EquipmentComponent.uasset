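; Actor component that manages a character's equipment as spawned item actors, starting from a configurable StartingEquipment class list.
; InitializeEquipment clears current items, then equips the starting set through EquipItem, which replaces any same-class item and spawns one owned by the component's owner.
; Gameplay tags select equipped items for lookup or to trigger their action.
; UnequipItem notifies and destroys the actor but leaves its EquippedItems entry, so tag searches check validity.
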(fn `EquipItem`
  (params (Equipment :type "/Game/CombatSystem/Blueprints/Actors/BP_BasicEquippable Class Reference"))
  (returns (`Success?` :type Boolean))
  (bind _returnvalue (`self.GetOwner`))
  (if (`KismetSystemLibrary.IsValidClass` Equipment)
    (`|ExecutionSequence`
      (:`then_0`
        (for _array_element (`self.EquippedItems`)
          (if (== (`GameplayStatics.GetObjectClass` _array_element) (`local.Equipment`))
            (`self.UnequipItem` _array_element))))
      (:`then_1`
        (bind _returnvalue_2 (`|SpawnActorFromClass` Equipment (`Actor.GetTransform` _returnvalue) "Undefined" "OverrideRootScale" _returnvalue (cast `Pawn` _returnvalue :!pure true)))
        (`/Game/CombatSystem/Blueprints/Actors/BP_BasicEquippable.OnEquipped` _returnvalue_2)
        (`KismetArrayLibrary.Array_AddUnique` (`self.EquippedItems`) _returnvalue_2)
        (return true)))
    (else
      (return false))))

(fn `GetEquippedItemByTag`
  (params (ItemTag :type "GameplayTag Structure"))
  (returns (ReturnValue :type "/Game/CombatSystem/Blueprints/Actors/BP_BasicEquippable Object Reference"))
  (for _array_element (`self.EquippedItems`)
    (`/Engine/EditorBlueprintResources/StandardMacros.IsValid` _array_element
      (:`Is Valid`
        (bind _returnvalue (`/Game/CombatSystem/Blueprints/Actors/BP_BasicEquippable.HasMatchingGameplayTag` _array_element ItemTag))
        (if _returnvalue
          (return _array_element))))))

(fn `InitializeEquipment`
  (`|ExecutionSequence`
    (:`then_0`
      (for _array_element (`self.EquippedItems`)
        (`self.UnequipItem` _array_element)))
    (:`then_1`
      (for _array_element_2 (`self.StartingEquipment`)
        (if (`KismetSystemLibrary.IsValidClass` _array_element_2)
          (`self.EquipItem` _array_element_2)))
      (return))))

(fn `PerformActionFromItem`
  (params (ItemTag :type "GameplayTag Structure"))
  (for _array_element (`self.EquippedItems`)
    (`/Engine/EditorBlueprintResources/StandardMacros.IsValid` _array_element
      (:`Is Valid`
        (bind _returnvalue (`/Game/CombatSystem/Blueprints/Actors/BP_BasicEquippable.HasMatchingGameplayTag` _array_element ItemTag))
        (if _returnvalue
          (`/Game/CombatSystem/Blueprints/Actors/BP_BasicEquippable.PerformItemAction` _array_element)
          (return)))))
  (return))

(fn `UnequipItem`
  (params (EquipmentToUnequip :type "/Game/CombatSystem/Blueprints/Actors/BP_BasicEquippable Object Reference"))
  (`/Engine/EditorBlueprintResources/StandardMacros.IsValid` EquipmentToUnequip
    (:`Is Valid`
      (`/Game/CombatSystem/Blueprints/Actors/BP_BasicEquippable.OnUnequipped` EquipmentToUnequip)
      (`Actor.K2_DestroyActor` (`local.EquipmentToUnequip`)))))