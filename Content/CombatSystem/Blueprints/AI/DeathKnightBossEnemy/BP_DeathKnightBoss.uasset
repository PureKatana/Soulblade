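; BP_DeathKnightBoss is a Death Knight boss enemy Blueprint that responds to its combat component's toggle event.
; On toggle, it snaps the weapon mesh to a socket on the character mesh and sends the combat type to the Anim Instance.
; The socket choice is fixed to false, so the weapon always goes to the attach socket, never the hand socket.
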(event `self.CombatComponent.OnCombatToggle`
  (params (`bIsCombatEnabled?` :type Boolean))
  (`SceneComponent.K2_AttachToComponent` (`self.WeaponMesh`) (`self.Mesh`) (select `bool` false :`false` (`self.Attach Socket Name`) :`true` (`self.Hand Socket Name`)) "SnapToTarget" "SnapToTarget" "SnapToTarget" true)
  (message `/Game/CombatSystem/Blueprints/Interfaces/AnimInstance_BPI.UpdateCombatType` (`SkeletalMeshComponent.GetAnimInstance` (`self.Mesh`)) (`self.Combat Type`)))

(fn `UserConstructionScript`
  (`parent.UserConstructionScript`))