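; Spear knight enemy Blueprint, a heavy mob whose spear changes socket and dissolve state as combat toggles.
; BeginPlay attaches the spear to a back socket and zeroes its material's Dissolve parameter.
; The CombatComponent's toggle event snaps the spear to the hand or attach socket and sends the combat type to the AnimInstance.
; It also fires a dissolve effect and runs a timeline forward or backward to drive that material parameter.
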(event `self.ReceiveBeginPlay`
  (bind _weaponmesh (`self.WeaponMesh`))
  (`parent.ReceiveBeginPlay`)
  (`SceneComponent.K2_AttachToComponent` (`self.WeaponMesh`) (`self.Mesh`) "SpearBackSocket" "KeepRelative" "KeepRelative" "KeepRelative" true)
  (bind _returnvalue (`PrimitiveComponent.CreateDynamicMaterialInstance` _weaponmesh 0 (`PrimitiveComponent.GetMaterial` _weaponmesh 0) "None"))
  (`MaterialInstanceDynamic.SetScalarParameterValue` _returnvalue "Dissolve" 0.0))

(event `self.CombatComponent.OnCombatToggle`
  (params (`bIsCombatEnabled?` :type Boolean))
  (bind _weaponmesh (`self.WeaponMesh`))
  (`SceneComponent.K2_AttachToComponent` (`self.WeaponMesh`) (`self.Mesh`) (select `bool` `bIsCombatEnabled?` :`false` (`self.Attach Socket Name`) :`true` (`self.Hand Socket Name`)) "SnapToTarget" "SnapToTarget" "SnapToTarget" true)
  (message `/Game/CombatSystem/Blueprints/Interfaces/AnimInstance_BPI.UpdateCombatType` (`SkeletalMeshComponent.GetAnimInstance` (`self.Mesh`)) (`self.Combat Type`))
  (if `bIsCombatEnabled?`
    (`ActorComponent.Activate` (`self.SpearWeaponDissolve_NS`) true)
    (bind (_direction _dissolve) (`Timeline|Dissolve` :!label _label)
      (:`Update`
        (bind _returnvalue (`PrimitiveComponent.CreateDynamicMaterialInstance` _weaponmesh 0 (`PrimitiveComponent.GetMaterial` _weaponmesh 0) "None"))
        (`MaterialInstanceDynamic.SetScalarParameterValue` _returnvalue "Dissolve" _dissolve)))
    (else
      (`ActorComponent.Activate` (`self.SpearWeaponDissolve_NS`) true)
      (goto _label :!via `Reverse`))))

(fn `UserConstructionScript`
  (`parent.UserConstructionScript`))