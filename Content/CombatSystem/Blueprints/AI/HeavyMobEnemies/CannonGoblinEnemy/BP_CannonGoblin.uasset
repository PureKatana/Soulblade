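; Cannon Goblin enemy Blueprint that extends a parent combat character with two melee weapon hitboxes and a floating health bar.
; Both weapon collision components feed one hit handler, which applies point damage scaled by the goblin's stats to actors that can receive it.
; The stats-bound health bar shows while targeted, or for a short delay after taking damage.
; On death, both weapon meshes switch to physics simulation.
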(event `self.ReceiveBeginPlay`
  (`parent.ReceiveBeginPlay`)
  (`/Game/CombatSystem/Blueprints/Components/CollisionComponent.SetCollisionMeshComponent` (`self.RightWeaponCollisionComponent`) (`self.RightWeaponMesh`))
  (`/Game/CombatSystem/Blueprints/Components/CollisionComponent.SetCollisionMeshComponent` (`self.LeftWeaponCollisionComponent`) (`self.LeftWeaponMesh`))
  (bind _returnvalue (`|CreateWidget` "/Game/CombatSystem/UI/W_Healthbar.W_Healthbar_C" (`GameplayStatics.GetPlayerController` 0) (`self.StatsComponent`)))
  (`WidgetComponent.SetWidget` (`self.HealthBar`) _returnvalue))

(event `/Game/CombatSystem/Blueprints/Interfaces/Targeting_BPI.OnTargeted`
  (params (`bIsTargeted?` :type Boolean))
  (`parent.OnTargeted` `bIsTargeted?`)
  (bind _output_get (set `self.Is Targeted?` `bIsTargeted?`))
  (`SceneComponent.SetVisibility` (`self.HealthBar`) _output_get false))

(event `self.RightWeaponCollisionComponent.OnHit`
  (params (`Hit Result` :type "HitResult Structure"))
  (`self.On Hit Event` `Hit Result`))

(event `self.LeftWeaponCollisionComponent.OnHit`
  (params (`Hit Result` :type "HitResult Structure"))
  (`self.On Hit Event` `Hit Result`))

(event `On Hit Event`
  (params (HitResult :type "HitResult Structure"))
  (bind (_bblockinghit _binitialoverlap _time _distance _location _impactpoint _normal _impactnormal _physmat _hitactor) (`GameplayStatics.BreakHitResult` HitResult))
  (bind _return_value (message `/Game/CombatSystem/Blueprints/Interfaces/CombatBPI.CanRecieveDamage` _hitactor))
  (if _return_value
    (`GameplayStatics.ApplyPointDamage` _hitactor (`/Game/CombatSystem/Blueprints/Components/StatsComponent.GetCurrentStatValue` (`self.StatsComponent`) "NewEnumerator3") (`self.GetActorForwardVector`) HitResult (`self.GetController`) self "/Game/CombatSystem/Blueprints/DamageTypes/BP_AttackDamageType.BP_AttackDamageType_C")))

(event `self.CombatComponent.OnCombatToggle`
  (params (`bIsCombatEnabled?` :type Boolean)))

(event `SimulateWeaponPhysics`
  (bind _leftweaponmesh (`self.LeftWeaponMesh`))
  (bind _rightweaponmesh (`self.RightWeaponMesh`))
  (`PrimitiveComponent.SetCollisionProfileName` _rightweaponmesh "PhysicsActor" true)
  (`PrimitiveComponent.SetSimulatePhysics` _rightweaponmesh true)
  (`PrimitiveComponent.SetCollisionProfileName` _leftweaponmesh "PhysicsActor" true)
  (`PrimitiveComponent.SetSimulatePhysics` _leftweaponmesh true))

(event `self.Death`
  (`parent.Death`)
  (`self.SimulateWeaponPhysics`))

(event `self.ReceivePointDamage`
  (params (Damage :type "Float (single-precision)") (DamageType :type "DamageType Object Reference") (HitLocation :type "Vector Structure") (HitNormal :type "Vector Structure") (HitComponent :type "PrimitiveComponent Object Reference") (BoneName :type Name) (ShotFromDirection :type "Vector Structure") (InstigatedBy :type "Controller Object Reference") (DamageCauser :type "Actor Object Reference") (HitInfo :type "HitResult Structure (by ref)"))
  (`self.ReceiveDamage` Damage DamageType InstigatedBy HitInfo HitLocation)
  (`SceneComponent.SetVisibility` (`self.HealthBar`) true false)
  (`KismetSystemLibrary.Delay` 1.0)
  (if (not (`self.Is Targeted?`))
    (`SceneComponent.SetVisibility` (`self.HealthBar`) false false)))

(fn `UserConstructionScript`
  (`parent.UserConstructionScript`))