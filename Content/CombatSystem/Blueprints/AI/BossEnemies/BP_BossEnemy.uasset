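; Boss enemy character that extends a parent enemy with a named on-screen health bar and combat music.
; Target acquisition registers it with the player, stops other detected enemies' music and shows the bar and music once, resetting on target loss.
; Left and right weapon collision components feed one hit handler applying stat-based point damage.
; Death hides the bar after a delay; a separate event drops the weapon with physics before destroying it.
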(event `self.ReceiveBeginPlay`
  (`parent.ReceiveBeginPlay`)
  (bind _returnvalue (`|CreateWidget` "/Game/CombatSystem/UI/W_BossHealth.W_BossHealth_C" (`GameplayStatics.GetPlayerController` 0)))
  (bind _output_get (set `self.BossHealthUI` _returnvalue))
  (`/Game/CombatSystem/UI/W_BossHealth.Initialize` _output_get (`self.StatsComponent`))
  (`/Game/CombatSystem/UI/W_BossHealth.SetBossName` (`self.BossHealthUI`) (`self.BossName`))
  (`UserWidget.AddToViewport` (`self.BossHealthUI`) 0))

(event `/Game/CombatSystem/Blueprints/Interfaces/Targeting_BPI.OnTargeted`
  (params (`bIsTargeted?` :type Boolean))
  (`parent.OnTargeted` `bIsTargeted?`))

(event `SetBossHealthVisibility`
  (params (`bVisible?` :type Boolean))
  (bind _bosshealthui (`self.BossHealthUI`)
    (:`then`
      (`Widget.SetVisibility` _bosshealthui (select `bool` `bVisible?` :`false` "Hidden" :`true` "Visible" :!type "ESlateVisibility Enum")))
    (:`else`)))

(event `self.RightWeaponCollisionComponent.OnHit`
  (params (`Hit Result` :type "HitResult Structure"))
  (`self.OnHitEvent` `Hit Result`))

(event `self.LeftWeaponCollisionComponent.OnHit`
  (params (`Hit Result` :type "HitResult Structure"))
  (`self.OnHitEvent` `Hit Result`))

(event `OnHitEvent`
  (params (`Hit Result` :type "HitResult Structure"))
  (bind (_bblockinghit _binitialoverlap _time _distance _location _impactpoint _normal _impactnormal _physmat _hitactor) (`GameplayStatics.BreakHitResult` `Hit Result`))
  (bind _return_value (message `/Game/CombatSystem/Blueprints/Interfaces/CombatBPI.CanRecieveDamage` _hitactor))
  (if _return_value
    (`GameplayStatics.ApplyPointDamage` _hitactor (`/Game/CombatSystem/Blueprints/Components/StatsComponent.GetCurrentStatValue` (`self.StatsComponent`) "NewEnumerator3") (`self.GetActorForwardVector`) `Hit Result` (`self.GetController`) self "/Game/CombatSystem/Blueprints/DamageTypes/BP_AttackDamageType.BP_AttackDamageType_C")))

(event `SimulateWeaponPhysics`
  (bind _weaponmesh (`self.WeaponMesh`))
  (`PrimitiveComponent.SetCollisionProfileName` _weaponmesh "PhysicsActor" true)
  (`PrimitiveComponent.SetSimulatePhysics` _weaponmesh true)
  (`KismetSystemLibrary.Delay` 2.0)
  (`ActorComponent.K2_DestroyComponent` _weaponmesh))

(event `self.Death`
  (`parent.Death`)
  (`KismetSystemLibrary.Delay` 5.98)
  (`self.SetBossHealthVisibility` false))

(event `self.OnTargetSet`
  (params (NewTarget :type "Actor Object Reference"))
  (bind _enemiesdetected (`/Game/GKnight/BP_PlayerCharacter.EnemiesDetected` (cast `/Game/GKnight/BP_PlayerCharacter` (`GameplayStatics.GetPlayerCharacter` 0) :!pure true)))
  (bind _output_get (set `self.TargetActor` NewTarget))
  (if (and (`KismetSystemLibrary.IsValid` _output_get) (!= (`/Game/CombatSystem/Blueprints/Components/StateManagerComponent.GetCurrentState` (`self.StateManagerComponent`)) (struct :`TagName` "Character.State.Dead")))
    (`KismetSystemLibrary.Delay` 0.05)
    (`/Engine/EditorBlueprintResources/StandardMacros.DoOnce` false :!label _label
      (:`Completed`
        (`KismetArrayLibrary.Array_Add` _enemiesdetected self)
        (for _array_element (`/Game/GKnight/BP_PlayerCharacter.EnemiesDetected` (cast `/Game/GKnight/BP_PlayerCharacter` (`GameplayStatics.GetPlayerCharacter` 0) :!pure true))
          (`AudioComponent.Stop` (`/Game/CombatSystem/Blueprints/AI/BP_MasterAI.CombatMusicComponent` _array_element)))
        (`self.PlayCombatMusic` true)
        (`self.SetBossHealthVisibility` true)))
    (else
      (`KismetArrayLibrary.Array_RemoveItem` _enemiesdetected self)
      (`self.SetBossHealthVisibility` false)
      (`self.PlayCombatMusic` false)
      (goto _label :!via `Reset`))))

(fn `UserConstructionScript`
  (`parent.UserConstructionScript`))