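; BP_SpiderQueen is the Spider Queen boss enemy, extending a parent class that supplies its base begin-play, death and construction logic.
; On BeginPlay it points the right and left weapon collision components at its own Mesh.
; On Death it runs the parent handling, waits about six seconds, then calls StartCutscene.
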(event `self.ReceiveBeginPlay`
  (`parent.ReceiveBeginPlay`)
  (`/Game/CombatSystem/Blueprints/Components/CollisionComponent.SetCollisionMeshComponent` (`self.RightWeaponCollisionComponent`) (`self.Mesh`))
  (`/Game/CombatSystem/Blueprints/Components/CollisionComponent.SetCollisionMeshComponent` (`self.LeftWeaponCollisionComponent`) (`self.Mesh`)))

(event `self.Death`
  (`parent.Death`)
  (`KismetSystemLibrary.Delay` 5.98)
  (`self.StartCutscene`))

(fn `UserConstructionScript`
  (`parent.UserConstructionScript`))