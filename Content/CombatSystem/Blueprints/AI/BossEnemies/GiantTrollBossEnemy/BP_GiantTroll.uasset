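; BP_GiantTroll is the giant troll boss enemy, extending a parent class that it calls on begin play, death and construction.
; On begin play it snaps its weapon mesh to the hand socket.
; The right weapon collision component uses that weapon mesh, while the left uses the character mesh.
; On death it calls SimulateWeaponPhysics before running the parent death logic.
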(event `self.ReceiveBeginPlay`
  (`parent.ReceiveBeginPlay`)
  (`SceneComponent.K2_AttachToComponent` (`self.WeaponMesh`) (`self.Mesh`) (`self.Hand Socket Name`) "SnapToTarget" "SnapToTarget" "SnapToTarget" true)
  (`/Game/CombatSystem/Blueprints/Components/CollisionComponent.SetCollisionMeshComponent` (`self.RightWeaponCollisionComponent`) (`self.WeaponMesh`))
  (`/Game/CombatSystem/Blueprints/Components/CollisionComponent.SetCollisionMeshComponent` (`self.LeftWeaponCollisionComponent`) (`self.Mesh`)))

(event `self.Death`
  (`self.SimulateWeaponPhysics`)
  (`parent.Death`))

(fn `UserConstructionScript`
  (`parent.UserConstructionScript`))