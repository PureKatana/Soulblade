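; BP_SwordSlash is a Death Knight boss slash effect that damages the player on contact.
; It registers itself as the Niagara system's callback handler and moves its Box collider to exported particle positions, so the hitbox follows the effect.
; On overlap, a player who can receive damage gets CostAllStamina set and takes point damage along the slash's forward vector.
; The delayed self-destroy logic is never executed.
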(event `self.ReceiveBeginPlay`
  (`NiagaraComponent.SetVariableObject` (`self.Niagara`) "SwordSlashCallbackHandler" self))

(event `self.ReceiveParticleData`
  (params (Data :type "Array of BasicParticleData Structure (by ref)") (NiagaraSystem :type "NiagaraSystem Object Reference") (SimulationPositionOffset :type "Vector Structure (by ref)"))
  (for _array_element Data
    (`SceneComponent.K2_SetRelativeLocation` (`self.Box`) (`.Position` (break `BasicParticleData` _array_element)) false false)))

(event `self.Box.OnComponentBeginOverlap`
  (params (OverlappedComponent :type "PrimitiveComponent Object Reference") (OtherActor :type "Actor Object Reference") (OtherComp :type "PrimitiveComponent Object Reference") (OtherBodyIndex :type Integer) (bFromSweep :type Boolean) (SweepResult :type "HitResult Structure (by ref)"))
  (bind _asbp_player_character (cast `/Game/GKnight/BP_PlayerCharacter` OtherActor))
  (bind _return_value (message `/Game/CombatSystem/Blueprints/Interfaces/CombatBPI.CanRecieveDamage` _asbp_player_character))
  (if _return_value
    (set `/Game/GKnight/BP_PlayerCharacter.bCostAllStamina?` true _asbp_player_character)
    (`GameplayStatics.ApplyPointDamage` _asbp_player_character (`self.Damage`) (`self.GetActorForwardVector`) SweepResult (`GameplayStatics.GetPlayerController` 0) self "/Game/CombatSystem/Blueprints/DamageTypes/BP_AttackDamageType.BP_AttackDamageType_C")))

(fn `UserConstructionScript`)