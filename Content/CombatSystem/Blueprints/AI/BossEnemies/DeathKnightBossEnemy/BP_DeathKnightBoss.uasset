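; BP_DeathKnightBoss is the Death Knight boss enemy Blueprint, extending its parent with weapon handling.
; On BeginPlay it registers the weapon mesh with the right weapon collision component.
; Toggling combat snaps the weapon between hand and attach sockets on the character mesh and sends the combat type to the anim instance.
; On death it simulates physics on the weapon before running the parent death logic.
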(event `self.ReceiveBeginPlay`
  (`parent.ReceiveBeginPlay`)
  (`/Game/CombatSystem/Blueprints/Components/CollisionComponent.SetCollisionMeshComponent` (`self.RightWeaponCollisionComponent`) (`self.WeaponMesh`)))

(event `self.CombatComponent.OnCombatToggle`
  (params (`bIsCombatEnabled?` :type Boolean))
  (`SceneComponent.K2_AttachToComponent` (`self.WeaponMesh`) (`self.Mesh`) (select `bool` `bIsCombatEnabled?` :`false` (`self.Attach Socket Name`) :`true` (`self.Hand Socket Name`)) "SnapToTarget" "SnapToTarget" "SnapToTarget" true)
  (message `/Game/CombatSystem/Blueprints/Interfaces/AnimInstance_BPI.UpdateCombatType` (`SkeletalMeshComponent.GetAnimInstance` (`self.Mesh`)) (`self.Combat Type`)))

(event `self.Death`
  (`self.SimulateWeaponPhysics`)
  (`parent.Death`))

(fn `UserConstructionScript`
  (`parent.UserConstructionScript`))