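; BP_MobEnemy is a weapon-wielding AI enemy with a floating stats-driven health bar, built on a parent that supplies targeting, damage and death logic.
; The combat toggle moves the weapon mesh between sockets and updates the animation's combat type.
; Weapon collision hits apply stat-based point damage to actors able to receive it.
; The health bar shows while targeted or briefly after damage, and the weapon turns physical on death.
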(event `self.ReceiveBeginPlay`
  (`parent.ReceiveBeginPlay`)
  (`/Game/CombatSystem/Blueprints/Components/CollisionComponent.SetCollisionMeshComponent` (`self.MainWeaponCollisionComponent`) (`self.WeaponMesh`))
  (bind _returnvalue (`|CreateWidget` "/Game/CombatSystem/UI/W_Healthbar.W_Healthbar_C" (`GameplayStatics.GetPlayerController` 0) (`self.StatsComponent`)))
  (`WidgetComponent.SetWidget` (`self.HealthBar`) _returnvalue))

(event `/Game/CombatSystem/Blueprints/Interfaces/Targeting_BPI.OnTargeted`
  (params (`bIsTargeted?` :type Boolean))
  (`parent.OnTargeted` `bIsTargeted?`)
  (bind _output_get (set `self.Is Targeted?` `bIsTargeted?`))
  (`SceneComponent.SetVisibility` (`self.HealthBar`) _output_get false))

(event `self.MainWeaponCollisionComponent.OnHit`
  (params (`Hit Result` :type "HitResult Structure"))
  (bind (_bblockinghit _binitialoverlap _time _distance _location _impactpoint _normal _impactnormal _physmat _hitactor) (`GameplayStatics.BreakHitResult` `Hit Result`))
  (bind _return_value (message `/Game/CombatSystem/Blueprints/Interfaces/CombatBPI.CanRecieveDamage` _hitactor))
  (if _return_value
    (`GameplayStatics.ApplyPointDamage` _hitactor (`/Game/CombatSystem/Blueprints/Components/StatsComponent.GetCurrentStatValue` (`self.StatsComponent`) "NewEnumerator3") (`self.GetActorForwardVector`) `Hit Result` (`self.GetController`) self "/Game/CombatSystem/Blueprints/DamageTypes/BP_AttackDamageType.BP_AttackDamageType_C")))

(event `self.CombatComponent.OnCombatToggle`
  (params (`bIsCombatEnabled?` :type Boolean))
  (`SceneComponent.K2_AttachToComponent` (`self.WeaponMesh`) (`self.Mesh`) (select `bool` `bIsCombatEnabled?` :`false` (`self.Attach Socket Name`) :`true` (`self.Hand Socket Name`)) "SnapToTarget" "SnapToTarget" "SnapToTarget" true)
  (message `/Game/CombatSystem/Blueprints/Interfaces/AnimInstance_BPI.UpdateCombatType` (`SkeletalMeshComponent.GetAnimInstance` (`self.Mesh`)) (`self.Combat Type`)))

(event `SimulateWeaponPhysics`
  (bind _weaponmesh (`self.WeaponMesh`))
  (`PrimitiveComponent.SetCollisionProfileName` _weaponmesh "PhysicsActor" true)
  (`PrimitiveComponent.SetSimulatePhysics` _weaponmesh true))

(event `self.Death`
  (`parent.Death`)
  (`self.SimulateWeaponPhysics`))

(event `self.ReceivePointDamage`
  (params (Damage :type "Float (single-precision)") (DamageType :type "DamageType Object Reference") (HitLocation :type "Vector Structure") (HitNormal :type "Vector Structure") (HitComponent :type "PrimitiveComponent Object Reference") (BoneName :type Name) (ShotFromDirection :type "Vector Structure") (InstigatedBy :type "Controller Object Reference") (DamageCauser :type "Actor Object Reference") (HitInfo :type "HitResult Structure (by ref)"))
  (`self.ReceiveDamage` Damage DamageType InstigatedBy HitInfo HitLocation)
  (`SceneComponent.SetVisibility` (`self.HealthBar`) true false)
  (`KismetSystemLibrary.Delay` 1.0)
  (if (not (`self.Is Targeted?`))
    (`SceneComponent.SetVisibility` (`self.HealthBar`) false false)))

(fn `UserConstructionScript`
  (`parent.UserConstructionScript`))