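; Blueprint Interface for the combat system, declaring the calls that combatant actors implement.
; It covers attack chaining and reset, attack and action execution by type or tag with duration and success results, and custom montage actions.
; Other functions toggle collision parts, i-frames and movement, drive rotation toward a target, report damage eligibility and movement speed mode, and update an item amount.
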(fn `ActivateCollision`
  (params (CollisionPart :type "/Game/CombatSystem/Blueprints/Enums/E_CollisionPart Enum" :default "NewEnumerator0")))

(fn `CanRecieveDamage`
  (returns (`Return Value` :type Boolean))
  (return false))

(fn `ContinueAttack`)

(fn `DeactivateCollision`
  (params (CollisionPart :type "/Game/CombatSystem/Blueprints/Enums/E_CollisionPart Enum" :default "NewEnumerator0")))

(fn `DisableMovement`
  (params (`bDisableMovement?` :type Boolean)))

(fn `GetDesiredRotation`
  (returns (`Return Value` :type "Rotator Structure"))
  (return))

(fn `GetMovementSpeedMode`
  (returns (ReturnValue :type "/Game/CombatSystem/Blueprints/Enums/E_MovementSpeedMode Enum"))
  (return "NewEnumerator0"))

(fn `PerformAction`
  (params (ActionTag :type "GameplayTag Structure") (StateTag :type "GameplayTag Structure" :default (struct :`TagName` "Character.State.General Action State")) (MontageIndex :type Integer) (bRandomIndex :type Boolean) (DamageType :type "/Game/CombatSystem/Blueprints/Enums/E_DamageType Enum" :default "NewEnumerator0"))
  (returns (ActionDuration :type "Float (double-precision)") (`bSuccess?` :type Boolean))
  (return 0.0 false))

(fn `PerformAttack`
  (params (AttackType :type "GameplayTag Structure") (AttackIndex :type Integer) (bRandomIndex :type Boolean))
  (returns (AttackDuration :type "Float (double-precision)") (`bSuccess?` :type Boolean))
  (return 0.0 false))

(fn `PerformCustomAction`
  (params (ActionTag :type "GameplayTag Structure") (StateTag :type "GameplayTag Structure") (Montage :type "AnimMontage Object Reference") (`bAutoReset?` :type Boolean) (MontagePlayRate :type "Float (double-precision)" :default 1.0))
  (returns (`bSuccess?` :type Boolean))
  (return false))

(fn `ResetAttack`)

(fn `ResetCombat`)

(fn `RotateToTarget`)

(fn `SetiFrames`
  (params (`bEnableiFrames?` :type Boolean)))

(fn `UpdateItemAmount`
  (params (Amount :type Integer)))