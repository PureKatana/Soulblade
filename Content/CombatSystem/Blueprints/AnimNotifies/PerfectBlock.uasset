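; Anim notify state that marks the perfect block window during a block animation.
; On begin, if the owner's CombatComponent reports perfect block is on, it enables the owner's perfect block message and switches the capsule to a custom collision object type.
; On end, it clears the message and restores the capsule to Pawn unconditionally.
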(fn `Received_NotifyBegin`
  (params (MeshComp :type "SkeletalMeshComponent Object Reference") (Animation :type "AnimSequenceBase Object Reference") (TotalDuration :type "Float (single-precision)") (EventReference :type "AnimNotifyEventReference Structure (by ref)"))
  (returns (ReturnValue :type Boolean))
  (bind _returnvalue (`ActorComponent.GetOwner` MeshComp))
  (if (`/Game/CombatSystem/Blueprints/Components/CombatComponent.IsPerfectBlockOn?` (`Actor.GetComponentByClass` _returnvalue "/Game/CombatSystem/Blueprints/Components/CombatComponent.CombatComponent_C"))
    (message `/Game/CombatSystem/Blueprints/Interfaces/CombatBPI.SetPerfectBlock` _returnvalue true)
    (`PrimitiveComponent.SetCollisionObjectType` (`Character.CapsuleComponent` (cast `Character` _returnvalue :!pure true)) "ECC_GameTraceChannel2")
    (return true)))

(fn `Received_NotifyEnd`
  (params (MeshComp :type "SkeletalMeshComponent Object Reference") (Animation :type "AnimSequenceBase Object Reference") (EventReference :type "AnimNotifyEventReference Structure (by ref)"))
  (returns (ReturnValue :type Boolean))
  (bind _returnvalue (`ActorComponent.GetOwner` MeshComp))
  (message `/Game/CombatSystem/Blueprints/Interfaces/CombatBPI.SetPerfectBlock` _returnvalue false)
  (`PrimitiveComponent.SetCollisionObjectType` (`Character.CapsuleComponent` (cast `Character` _returnvalue :!pure true)) "ECC_Pawn")
  (return true))