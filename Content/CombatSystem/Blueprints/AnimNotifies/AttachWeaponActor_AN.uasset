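; AttachWeaponActor_AN is an anim notify that moves the player's main weapon and shield between hand and attach sockets during an animation.
; It runs only for BP_PlayerCharacter owners and gets the main weapon from their CombatComponent.
; The AttachToHand flag picks each item's socket for its attach call.
; The shield, read from the character, is attached only when a valid main weapon exists.
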(fn `Received_Notify`
  (params (MeshComp :type "SkeletalMeshComponent Object Reference") (Animation :type "AnimSequenceBase Object Reference") (EventReference :type "AnimNotifyEventReference Structure (by ref)"))
  (returns (ReturnValue :type Boolean))
  (bind _returnvalue (`ActorComponent.GetOwner` MeshComp))
  (bind _return_value (`/Game/CombatSystem/Blueprints/Components/CombatComponent.GetMainWeapon` (`Actor.GetComponentByClass` _returnvalue "/Game/CombatSystem/Blueprints/Components/CombatComponent.CombatComponent_C")))
  (bind _asbp_player_character (cast `/Game/CombatSystem/Blueprints/BP_PlayerCharacter` _returnvalue))
  (`/Engine/EditorBlueprintResources/StandardMacros.IsValid` _return_value
    (:`Is Valid`
      (`/Game/CombatSystem/Blueprints/Actors/BP_BasicEquippable.AttachActor` _return_value (select `bool` (`self.AttachToHand`) :`false` (`/Game/CombatSystem/Blueprints/Actors/BP_BasicEquippable.Attach Socket Name` _return_value) :`true` (`/Game/CombatSystem/Blueprints/Actors/BP_BaseWeapon.HandSocketName` _return_value)))
      (bind _return_value_2 (`/Game/CombatSystem/Blueprints/BP_PlayerCharacter.GetShield` _asbp_player_character))
      (`/Engine/EditorBlueprintResources/StandardMacros.IsValid` _return_value_2
        (:`Is Valid`
          (`/Game/CombatSystem/Blueprints/Actors/BP_Sword_Shield.AttachShield` _return_value_2 (select `bool` (`self.AttachToHand`) :`false` (`/Game/CombatSystem/Blueprints/Actors/BP_Sword_Shield.ShieldAttachSocket` _return_value_2) :`true` (`/Game/CombatSystem/Blueprints/Actors/BP_Sword_Shield.ShieldHandSocket` _return_value_2)))
          (return false))
        (:`Is Not Valid`
          (return false))))))