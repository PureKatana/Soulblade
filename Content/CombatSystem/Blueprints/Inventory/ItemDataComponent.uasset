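; Actor component that makes its owner a pickup item, carrying an item ID row reference and a quantity.
; On Interact, it casts the caller to BP_PlayerCharacter and passes the row name and quantity to that character's InventorySystem through AddToInventory.
; The owning actor is destroyed only when the add succeeds, with debug prints for interaction, invalid inventory and failed cast.
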(event `/Game/CombatSystem/Blueprints/Interfaces/Interactable_BPI.Interact`
  (params (Caller :type "Actor Object Reference"))
  (bind (_itemid_datatable _itemid_rowname) (break `DataTableRowHandle` (`self.ItemID`)))
  (bind _asbp_player_character (cast `/Game/GKnight/BP_PlayerCharacter` Caller)
    (:`then`
      (bind _inventorysystem (`/Game/GKnight/BP_PlayerCharacter.InventorySystem` _asbp_player_character))
      (`/Engine/EditorBlueprintResources/StandardMacros.IsValid` _inventorysystem
        (:`Is Valid`
          (bind _success (`/Game/CombatSystem/Blueprints/Inventory/InventorySystem.AddToInventory` _inventorysystem _itemid_rowname (`self.Quantity`)))
          (if _success
            (`KismetSystemLibrary.PrintString` "interacted")
            (`Actor.K2_DestroyActor` (`self.GetOwner`))))
        (:`Is Not Valid`
          (`KismetSystemLibrary.PrintString` "not valid"))))
    (:`CastFailed`
      (`KismetSystemLibrary.PrintString` "failed"))))