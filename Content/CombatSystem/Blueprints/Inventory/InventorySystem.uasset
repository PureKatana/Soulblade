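; Slot-based inventory that stores item IDs and quantities in a Content array sized to InventorySize on BeginPlay.
; AddToInventory places items one unit at a time, filling matching stacks up to the ItemData table's StackSize, then claiming empty slots.
; It reports success and the leftover quantity when space runs out.
; RemoveFromInventory is an empty stub, and key 4 prints every slot for debugging.
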(event `self.ReceiveBeginPlay`
  (`KismetArrayLibrary.Array_Resize` (`self.Content`) (`self.InventorySize`)))

(event `Key|Four`
  (params (Key :type "Key Structure"))
  (:`Pressed`
    (`self.DEBUG`)))

(fn `AddToInventory`
  (params (ItemID :type Name) (Quantity :type Integer))
  (returns (success :type Boolean) (`quantity remaining` :type Integer))
  (locals (`Local Quantity Remaining` :type Integer) (`Local Has Failed` :type Boolean))
  (set `local.Local Quantity Remaining` Quantity)
  (while (and (> (`local.Local Quantity Remaining`) 0) (not (`local.Local Has Failed`)))
    (bind (_index _foundslot) (`self.FindSlot` (`local.ItemID`)))
    (if _foundslot
      (`self.AddToStack` _index 1)
      (`/Engine/EditorBlueprintResources/StandardMacros.DecrementInt` (`local.Local Quantity Remaining`))
      (elif (`self.AnyEmptySlotsAvailable`)
        (bind _success (`self.CreateNewStack` (`local.ItemID`) 1))
        (if _success
          (`/Engine/EditorBlueprintResources/StandardMacros.DecrementInt` (`local.Local Quantity Remaining`))
          (else
            (set `local.Local Has Failed` true)))
        (else
          (set `local.Local Has Failed` true)
          (`KismetSystemLibrary.PrintString` "local failed 1")))))
  (return (not (`local.Local Has Failed`)) (`local.Local Quantity Remaining`)))

(fn `AddToStack`
  (params (index :type Integer) (quantity :type Integer))
  (bind (_output_itemid _output_quantity) (break `/Game/CombatSystem/Blueprints/Inventory/FSlot` (`|GetArrayItem` (`self.Content`) index)))
  (`KismetArrayLibrary.Array_Set` (`self.Content`) index (make `/Game/CombatSystem/Blueprints/Inventory/FSlot` _output_itemid (+ _output_quantity (`local.quantity`)))))

(fn `AnyEmptySlotsAvailable`
  (returns (HasEmptySlot :type Boolean) (EmptyIndex :type Integer))
  (for (_array_element _array_index) (`self.Content`)
    (if (== (`.quantity_5_A891AF254918C65CF33356B23861EF4F` (break `/Game/CombatSystem/Blueprints/Inventory/FSlot` _array_element)) 0)
      (return true _array_index)))
  (return false -1))

(fn `CreateNewStack`
  (params (ItemID :type Name) (Quantity :type Integer))
  (returns (success :type Boolean))
  (bind (_hasemptyslot _emptyindex) (`self.AnyEmptySlotsAvailable`))
  (if _hasemptyslot
    (`KismetArrayLibrary.Array_Set` (`self.Content`) _emptyindex (make `/Game/CombatSystem/Blueprints/Inventory/FSlot` (`local.ItemID`) (`local.Quantity`)))
    (return true)
    (else
      (return false))))

(fn `DEBUG`
  (for (_array_element _array_index) (`self.Content`)
    (bind (_itemid _quantity) (break `/Game/CombatSystem/Blueprints/Inventory/FSlot` _array_element))
    (`KismetSystemLibrary.PrintString` (`KismetStringLibrary.Concat_StrStr` (`KismetStringLibrary.Conv_IntToString` _array_index) " - " (`KismetStringLibrary.Conv_NameToString` _itemid) " | " (`KismetStringLibrary.Conv_IntToString` _quantity)))))

(fn `FindSlot`
  (params (ItemID :type Name))
  (returns (index :type Integer) (foundslot :type Boolean))
  (bind _itemid (`local.ItemID`))
  (for (_array_element _array_index) (`self.Content`)
    (bind (_itemid_2 _quantity) (break `/Game/CombatSystem/Blueprints/Inventory/FSlot` _array_element))
    (if (== _itemid_2 _itemid)
      (if (< _quantity (`self.GetMaxStackSize` _itemid))
        (return _array_index true))))
  (return -1 false))

(fn `GetMaxStackSize`
  (params (ItemID :type Name))
  (returns (StackSize :type Integer))
  (bind _returnvalue (`|GetDataTableRow` "/Game/CombatSystem/Blueprints/Inventory/ItemData.ItemData" ItemID)
    (:`then`
      (return (`.StackSize_14_85447EED4B92D34F9ECA02B12F7B9586` (break `/Game/CombatSystem/Blueprints/Inventory/FItemStruct` _returnvalue))))
    (:`RowNotFound`
      (return -1))))

(fn `RemoveFromInventory`)