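; Base Blueprint for weapons in the combat system, handling what happens when a weapon is equipped.
; OnEquipped runs the parent logic, then attaches the weapon to the hand socket or the attach socket, depending on whether the owner's CombatComponent has combat enabled.
; It registers itself as that component's main weapon and sends its CombatType to the owning Character's AnimInstance through a message call.
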(fn `OnEquipped`
  (`parent.OnEquipped`)
  (set `self.CombatComponent_C` (`self.GetComponentByClass` (`self.GetOwner`) "/Game/CombatSystem/Blueprints/Components/CombatComponent.CombatComponent_C"))
  (`self.AttachActor` (select `bool` (`/Game/CombatSystem/Blueprints/Components/CombatComponent.IsCombatEnabled?` (`self.CombatComponent_C`)) :`false` (`self.Attach Socket Name`) :`true` (`self.HandSocketName`)))
  (`/Game/CombatSystem/Blueprints/Components/CombatComponent.SetMainWeapon` (`self.CombatComponent_C`) self)
  (message `/Game/CombatSystem/Blueprints/Interfaces/AnimInstance_BPI.UpdateCombatType` (`SkeletalMeshComponent.GetAnimInstance` (`Character.Mesh` (cast `Character` (`self.GetOwner`) :!pure true))) (`self.CombatType`)))

(fn `UserConstructionScript`
  (`parent.UserConstructionScript`))