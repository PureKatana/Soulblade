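; BP_PickupActor is an interactable pickup that gives the interacting character an item, such as a weapon.
; A Sphere overlap with the player character shows or hides the interact prompt on the BP_PlayerController's MainHUD.
; Interact calls EquipWeapon, which spawns the Item class at the pickup's transform with the caller as owner and instigator, then calls OnEquipped on it.
; The pickup does not destroy itself afterwards.
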(event `/Game/CombatSystem/Blueprints/Interfaces/Interactable_BPI.Interact`
  (params (Caller :type "Actor Object Reference"))
  (`self.EquipWeapon` Caller Caller))

(event `self.Sphere.OnComponentBeginOverlap`
  (params (OverlappedComponent :type "PrimitiveComponent Object Reference") (OtherActor :type "Actor Object Reference") (OtherComp :type "PrimitiveComponent Object Reference") (OtherBodyIndex :type Integer) (bFromSweep :type Boolean) (SweepResult :type "HitResult Structure (by ref)"))
  (if (== OtherActor (`GameplayStatics.GetPlayerCharacter` 0))
    (bind _asbp_player_controller (cast `/Game/CombatSystem/Blueprints/BP_PlayerController` (`GameplayStatics.GetPlayerController` 0)))
    (`/Game/CombatSystem/UI/W_MainHUD.ShowInteractText` (`/Game/CombatSystem/Blueprints/BP_PlayerController.MainHUD` _asbp_player_controller))))

(event `self.Sphere.OnComponentEndOverlap`
  (params (OverlappedComponent :type "PrimitiveComponent Object Reference") (OtherActor :type "Actor Object Reference") (OtherComp :type "PrimitiveComponent Object Reference") (OtherBodyIndex :type Integer))
  (if (== OtherActor (`GameplayStatics.GetPlayerCharacter` 0))
    (bind _asbp_player_controller (cast `/Game/CombatSystem/Blueprints/BP_PlayerController` (`GameplayStatics.GetPlayerController` 0)))
    (`/Game/CombatSystem/UI/W_MainHUD.HideInteractText` (`/Game/CombatSystem/Blueprints/BP_PlayerController.MainHUD` _asbp_player_controller))))

(fn `EquipWeapon`
  (params (Owner :type "Actor Object Reference") (Object :type "Object Object Reference"))
  (bind _returnvalue (`|SpawnActorFromClass` (`self.Item`) (`self.GetTransform`) "Undefined" "OverrideRootScale" Owner (cast `Pawn` Object :!pure true)))
  (`/Game/CombatSystem/Blueprints/Actors/BP_BasicEquippable.OnEquipped` _returnvalue))

(fn `UserConstructionScript`)