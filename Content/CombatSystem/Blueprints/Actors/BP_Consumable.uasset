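; BP_Consumable is a usable item actor with limited charges that modifies one of its owner's stats, refilled to its maximum on BeginPlay.
; PerformItemAction checks for remaining uses, then messages the owner to play the use montage as a tagged UseItem action.
; ConsumeItem separately decrements the count, reports it to the owner and applies the modification through the owner's StatsComponent, with optional regeneration.
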(event `self.ReceiveBeginPlay`
  (`parent.ReceiveBeginPlay`)
  (`self.SetCurrentNumberOfUses`))

(event `self.PerformItemAction`
  (if (> (`self.CurrentNumberOfUses`) 0)
    (message `/Game/CombatSystem/Blueprints/Interfaces/CombatBPI.PerformCustomAction` (`self.GetOwner`) (struct :`TagName` "Character.Action.UseItem") (struct :`TagName` "Character.State.General Action State") (`self.UseItemMontage`) false 1.0)))

(event `ConsumeItem`
  (bind _result (`/Engine/EditorBlueprintResources/StandardMacros.DecrementInt` (`self.CurrentNumberOfUses`))
    (:`  `
      (message `/Game/CombatSystem/Blueprints/Interfaces/CombatBPI.UpdateItemAmount` (`self.GetOwner`) _result)
      (`/Game/CombatSystem/Blueprints/Components/StatsComponent.ModifyCurrentStatValue` (`self.GetComponentByClass` (`self.GetOwner`) "/Game/CombatSystem/Blueprints/Components/StatsComponent.StatsComponent_C") (`self.Stats`) (`self.ModificationValue`) (`self.Should Regenerate?`)))))

(fn `SetCurrentNumberOfUses`
  (set `self.CurrentNumberOfUses` (`self.MaxNumberOfUses`)))

(fn `UserConstructionScript`
  (`parent.UserConstructionScript`))