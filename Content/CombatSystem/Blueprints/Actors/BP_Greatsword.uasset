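; BP_Greatsword is a greatsword weapon actor that changes how it is held when its owner blocks.
; On BeginPlay it runs the parent logic, then binds to the block-set event on the owner's CombatComponent.
; When that event fires, it re-attaches itself to GreatswordHandBlockSocket while blocking, or to its regular HandSocketName socket otherwise.
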(event `self.ReceiveBeginPlay`
  (`parent.ReceiveBeginPlay`)
  (add `/Game/CombatSystem/Blueprints/Components/CombatComponent.OnBlockSet` (`self.GetComponentByClass` (`self.GetOwner`) "/Game/CombatSystem/Blueprints/Components/CombatComponent.CombatComponent_C") (delegate `AttachGreatswordToBlockHand`)))

(event `AttachGreatswordToBlockHand`
  (params (`bIsBlocking?` :type Boolean))
  (set `self.bIsBlocking?` `bIsBlocking?`)
  (`self.AttachActor` (select `bool` (`self.bIsBlocking?`) :`false` (`self.HandSocketName`) :`true` (`self.GreatswordHandBlockSocket`))))

(fn `UserConstructionScript`
  (`parent.UserConstructionScript`))