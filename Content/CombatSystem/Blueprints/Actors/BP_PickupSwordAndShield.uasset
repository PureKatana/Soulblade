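; BP_PickupSwordAndShield is an interactable pickup that equips the player with a sword and shield.
; On Interact, it spawns its Item class at its own transform, owned and instigated by the caller, then calls OnEquipped.
; If that item is a BP_SwordAndShield, it registers it as the shield on player 0's character, rather than the caller, and attaches the shield to ShieldAttachSocket.
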(event `/Game/CombatSystem/Blueprints/Interfaces/Interactable_BPI.Interact`
  (params (Caller :type "Actor Object Reference"))
  (bind _returnvalue (`|SpawnActorFromClass` (`self.Item`) (`self.GetTransform`) "Undefined" "OverrideRootScale" Caller (cast `Pawn` Caller :!pure true)))
  (`/Game/CombatSystem/Blueprints/Actors/BP_BasicEquippable.OnEquipped` _returnvalue)
  (bind _asbp_player_character (cast `/Game/CombatSystem/Blueprints/BP_PlayerCharacter` (`GameplayStatics.GetPlayerCharacter` 0)))
  (bind _asbp_sword_shield (cast `/Game/CombatSystem/Blueprints/Actors/BP_SwordAndShield` _returnvalue))
  (`/Game/CombatSystem/Blueprints/BP_PlayerCharacter.SetShield` _asbp_player_character _asbp_sword_shield)
  (`/Game/CombatSystem/Blueprints/Actors/BP_SwordAndShield.AttachShield` _asbp_sword_shield "ShieldAttachSocket"))

(fn `UserConstructionScript`
  (`parent.UserConstructionScript`))