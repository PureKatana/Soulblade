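; Player controller for the GKnight game that owns the main HUD and background music.
; On BeginPlay it creates W_MainHUD and adds it to the viewport, then forwards item amount and zone text updates to it.
; It stores a music asset through getter and setter functions and plays or stops it on a music component.
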(event `self.ReceiveBeginPlay`
  (bind _returnvalue (`|CreateWidget` "/Game/CombatSystem/UI/W_MainHUD.W_MainHUD_C" self))
  (bind _output_get (set `self.MainHUD` _returnvalue))
  (`UserWidget.AddToViewport` _output_get 0))

(event `SetItemAmount`
  (params (Amount :type Integer))
  (bind _mainhud (`self.MainHUD`)
    (:`then`
      (`/Game/CombatSystem/UI/W_MainHUD.SetItemAmountText` _mainhud Amount))
    (:`else`)))

(event `SetZoneText`
  (params (InText :type Text))
  (bind _mainhud (`self.MainHUD`)
    (:`then`
      (`/Game/CombatSystem/UI/W_MainHUD.SetZoneText` _mainhud InText))
    (:`else`)))

(event `PlayMusic`
  (bind _music (`self.GetMusic`))
  (bind _musiccomponent (`self.MusicComponent`))
  (`/Engine/EditorBlueprintResources/StandardMacros.IsValid` _music
    (:`Is Valid`
      (`AudioComponent.SetSound` _musiccomponent _music)
      (`AudioComponent.Play` _musiccomponent 0.0))))

(event `StopMusic`
  (bind _musiccomponent (`self.MusicComponent`))
  (`/Engine/EditorBlueprintResources/StandardMacros.IsValid` _musiccomponent
    (:`Is Valid`
      (`AudioComponent.Stop` _musiccomponent))))

(fn `GetMusic`
  (returns (Music :type "SoundBase Object Reference"))
  (return (`self.Music`)))

(fn `SetMusic`
  (params (NewMusic :type "SoundBase Object Reference"))
  (set `self.Music` NewMusic))

(fn `UserConstructionScript`)