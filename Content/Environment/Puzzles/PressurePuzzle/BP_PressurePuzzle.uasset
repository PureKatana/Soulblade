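; Pressure-stone puzzle actor that opens its linked Door when the player triggers the stones in the correct sequence.
; The construction script builds a row of random stone meshes, each with an overlap box tagged by one RandomOrder character.
; Overlaps from a player holding at least one soul fragment append each stone's tag once.
; A full-length input is checked against CorrectOrder, playing success or failure sounds and resetting on failure.
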(fn `AddOrder`
  (params (Add :type String) (StoneActor :type "PrimitiveComponent Object Reference"))
  (if (not (`KismetArrayLibrary.Array_Contains` (`self.Stones`) StoneActor))
    (`KismetArrayLibrary.Array_AddUnique` (`self.Stones`) StoneActor)
    (set `self.OrderInput` (`KismetStringLibrary.Concat_StrStr` (`self.OrderInput`) Add))
    (`GameplayStatics.PlaySoundAtLocation` "/Game/Environment/Puzzles/PressurePuzzle/PressStone.PressStone" (`self.K2_GetActorLocation`) (struct) 0.5 1.0 0.0 null null null null)
    (if (== (`KismetStringLibrary.Len` (`self.CorrectOrder`)) (`KismetStringLibrary.Len` (`self.OrderInput`)))
      (if (== (`self.CorrectOrder`) (`self.OrderInput`))
        (message `/Game/Environment/Puzzles/Interfaces/Puzzle_BPI.OpenDoor` (`self.Door`))
        (`GameplayStatics.PlaySoundAtLocation` "/Game/Environment/Puzzles/SoundFX/Positive_Effect_10.Positive_Effect_10" (`self.K2_GetActorLocation`) (struct) 0.5 1.0 0.0 null null null null)
        (else
          (set `self.OrderInput` "")
          (`KismetArrayLibrary.Array_Clear` (`self.Stones`))
          (`GameplayStatics.PlaySoundAtLocation` "/Game/Environment/Puzzles/SoundFX/Negative_Effect_12.Negative_Effect_12" (`self.K2_GetActorLocation`) (struct) 0.5 1.0 0.0 null null null null))))))

(fn `BP_PressurePuzzle_AutoGenFunc`
  (params (OverlappedComponent :type "PrimitiveComponent Object Reference") (OtherActor :type "Actor Object Reference") (OtherComp :type "PrimitiveComponent Object Reference") (OtherBodyIndex :type Integer) (bFromSweep :type Boolean) (SweepResult :type "HitResult Structure (by ref)"))
  (bind _asbp_player_character (cast `/Game/GKnight/BP_PlayerCharacter` OtherActor))
  (if (>= (`/Game/GKnight/BP_PlayerCharacter.GetNumberOfSoulFragments` _asbp_player_character) 1)
    (`self.AddOrder` (`KismetStringLibrary.Conv_NameToString` (`|GetArrayItem` (`ActorComponent.ComponentTags` OverlappedComponent))) OverlappedComponent)
    (return)))

(fn `UserConstructionScript`
  (for _index (range (`KismetStringLibrary.Len` (`self.CorrectOrder`)))
    (bind _returnvalue (`AddComponent|NODE_AddStaticMeshComponent-0` :`RelativeTransform` (`KismetMathLibrary.MakeTransform` (`KismetMathLibrary.MakeVector` (* _index (`self.Spacing`))) (struct) (2.0 2.0 2.0))))
    (`StaticMeshComponent.SetStaticMesh` _returnvalue (`KismetArrayLibrary.Array_Random` (`self.StoneMeshes`)))
    (bind _returnvalue_2 (`AddComponent|NODE_AddBoxComponent-0` :`RelativeTransform` (`KismetMathLibrary.MakeTransform` (+ (`SceneComponent.RelativeLocation` _returnvalue) (0.0 0.0 40.0)))))
    (set `ActorComponent.ComponentTags` (`|MakeArray` (`KismetStringLibrary.Conv_StringToName` (`KismetStringLibrary.GetSubstring` (`self.RandomOrder`) _index))) _returnvalue_2)
    (add `PrimitiveComponent.OnComponentBeginOverlap` _returnvalue_2 (`|CreateDelegate` :!event `BP_PressurePuzzle_AutoGenFunc`))))