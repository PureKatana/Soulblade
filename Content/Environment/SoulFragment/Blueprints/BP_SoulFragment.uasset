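; Soul fragment actor that grants the player a fragment and can trigger a first-fragment cutscene.
; AddSoulFragment increments the player character's fragment count and calls LevelUpPlayer.
; Player overlap with the box broadcasts StartCutscene once, if the character allows the first cutscene.
; Separate events toggle the Niagara effect and destroy the actor after a delay; none are called within this graph.
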(event `AddSoulFragment`
  (bind _asbp_player_character (cast `/Game/GKnight/BP_PlayerCharacter` (`GameplayStatics.GetPlayerCharacter` 0)))
  (bind _result (`/Engine/EditorBlueprintResources/StandardMacros.IncrementInt` (`/Game/GKnight/BP_PlayerCharacter.GetNumberOfSoulFragments` _asbp_player_character))
    (:`  `
      (`/Game/GKnight/BP_PlayerCharacter.SetNumberOfSoulsFragments` _asbp_player_character _result)
      (`/Game/GKnight/BP_PlayerCharacter.LevelUpPlayer` _asbp_player_character))))

(event `Deactivate`
  (`ActorComponent.Deactivate` (`self.Niagara`)))

(event `Activate`
  (`ActorComponent.Activate` (`self.Niagara`) false))

(event `self.Box.OnComponentBeginOverlap`
  (params (OverlappedComponent :type "PrimitiveComponent Object Reference") (OtherActor :type "Actor Object Reference") (OtherComp :type "PrimitiveComponent Object Reference") (OtherBodyIndex :type Integer) (bFromSweep :type Boolean) (SweepResult :type "HitResult Structure (by ref)"))
  (cast `/Game/GKnight/BP_PlayerCharacter` OtherActor)
  (if (`/Game/GKnight/BP_PlayerCharacter.CanStartFirstSoulFragmentCutscene?` (cast `/Game/GKnight/BP_PlayerCharacter` (`GameplayStatics.GetPlayerCharacter` 0) :!pure true))
    (`/Engine/EditorBlueprintResources/StandardMacros.DoOnce` false
      (:`Completed`
        (`self.StartCutscene`)))))

(event `Destroy`
  (`KismetSystemLibrary.Delay` 5.0)
  (`self.K2_DestroyActor`))

(fn `UserConstructionScript`)