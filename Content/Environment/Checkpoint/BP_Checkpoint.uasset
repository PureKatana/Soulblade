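; Interactable checkpoint actor with a floating sword, spun by a looping timer and moved back and forth by a timeline.
; A sphere overlap shows or hides the HUD interact prompt for the player, and leaving resets the DoOnce gate.
; Interacting with no detected enemies stores the checkpoint as the player's position, heals, refills equipped consumables and plays burst effects, once per visit.
; Otherwise it displays combat text.
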(event `self.ReceiveBeginPlay`
  (`KismetSystemLibrary.K2_SetTimerDelegate` (delegate `RotateSword`) 0.005 true)
  (bind (_direction _newtrack_0) (`Timeline|Move` :!label _label)
    (:`Update`
      (`SceneComponent.K2_SetRelativeLocation` (`self.Sword`) _newtrack_0 false false)
      (`KismetSystemLibrary.Delay` 3.0)
      (if (`self.bIsLooped?`)
        (set `self.bIsLooped?` false)
        (goto _label :!via `Reverse`)
        (else
          (set `self.bIsLooped?` true)
          (goto _label))))))

(event `RotateSword`
  (bind _sword (`self.Sword`))
  (bind (_relativerotation_roll _relativerotation_pitch _relativerotation_yaw) (`KismetMathLibrary.BreakRotator` (`SceneComponent.RelativeRotation` _sword)))
  (`SceneComponent.K2_SetRelativeRotation` _sword (`KismetMathLibrary.MakeRotator` _relativerotation_roll _relativerotation_pitch (+ _relativerotation_yaw 1.0)) false false))

(event `self.Sphere.OnComponentBeginOverlap`
  (params (OverlappedComponent :type "PrimitiveComponent Object Reference") (OtherActor :type "Actor Object Reference") (OtherComp :type "PrimitiveComponent Object Reference") (OtherBodyIndex :type Integer) (bFromSweep :type Boolean) (SweepResult :type "HitResult Structure (by ref)"))
  (if (== OtherActor (`GameplayStatics.GetPlayerCharacter` 0))
    (bind _asbp_player_controller (cast `/Game/GKnight/BP_PlayerController` (`GameplayStatics.GetPlayerController` 0)))
    (`/Game/CombatSystem/UI/W_MainHUD.ShowInteractText` (`/Game/GKnight/BP_PlayerController.MainHUD` _asbp_player_controller))))

(event `self.Sphere.OnComponentEndOverlap`
  (params (OverlappedComponent :type "PrimitiveComponent Object Reference") (OtherActor :type "Actor Object Reference") (OtherComp :type "PrimitiveComponent Object Reference") (OtherBodyIndex :type Integer))
  (if (== OtherActor (`GameplayStatics.GetPlayerCharacter` 0))
    (bind _asbp_player_controller (cast `/Game/GKnight/BP_PlayerController` (`GameplayStatics.GetPlayerController` 0)))
    (`/Game/CombatSystem/UI/W_MainHUD.HideInteractText` (`/Game/GKnight/BP_PlayerController.MainHUD` _asbp_player_controller))
    (goto _label_2 :!via `Reset`)))

(event `/Game/CombatSystem/Blueprints/Interfaces/Interactable_BPI.Interact`
  (params (Caller :type "Actor Object Reference"))
  (bind _asbp_player_character (cast `/Game/GKnight/BP_PlayerCharacter` Caller))
  (bind _output_get (set `self.PlayerCharacter` _asbp_player_character))
  (if (`KismetArrayLibrary.Array_IsEmpty` (`/Game/GKnight/BP_PlayerCharacter.EnemiesDetected` _output_get))
    (`/Engine/EditorBlueprintResources/StandardMacros.DoOnce` false :!label _label_2
      (:`Completed`
        (set `/Game/GKnight/BP_PlayerCharacter.PlayerPosition` (`KismetMathLibrary.MakeTransform` (`self.K2_GetActorLocation`) (`self.K2_GetActorRotation`)) _output_get)
        (`/Game/GKnight/BP_PlayerCharacter.Heal` (`self.PlayerCharacter`))
        (for _array_element (`/Game/CombatSystem/Blueprints/Components/EquipmentComponent.GetEquippedItemsByTag` (`/Game/GKnight/BP_PlayerCharacter.EquipmentComponent` (`self.PlayerCharacter`)) (struct :`TagName` "Item.Consumable"))
          (bind _asbp_consumable (cast `/Game/CombatSystem/Blueprints/Actors/BP_Consumable` _array_element))
          (`/Game/CombatSystem/Blueprints/Actors/BP_Consumable.SetCurrentNumberOfUses` _asbp_consumable)
          (`/Game/GKnight/BP_PlayerCharacter.UpdateItemAmount` (`self.PlayerCharacter`) (`/Game/CombatSystem/Blueprints/Actors/BP_Consumable.MaxNumberOfUses` _asbp_consumable)))
        (`GameplayStatics.PlaySoundAtLocation` "/Game/Environment/Checkpoint/Pad_3_1.Pad_3_1" (`self.K2_GetActorLocation`) (struct) 0.5 1.0 0.0 null null null null)
        (`NiagaraFunctionLibrary.SpawnSystemAtLocation` "/Game/Environment/Checkpoint/CheckpointBurst_N.CheckpointBurst_N" (`self.K2_GetActorLocation`) (`self.K2_GetActorRotation`))))
    (else
      (`/Game/GKnight/BP_PlayerController.SetCombatText` (cast `/Game/GKnight/BP_PlayerController` (`GameplayStatics.GetPlayerController` 0) :!pure true)))))

(fn `UserConstructionScript`)