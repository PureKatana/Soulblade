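; BP_Rain is a rain actor that follows the player and draws small disturbances into a fluid simulation where rain particles report.
; A looping half-second timer is set up, and the Raining event repositions the actor high above the player character.
; The Rain effect passes particle data back to the Blueprint, which draws randomly sized, randomly strong splats through a dynamic draw material, skipping particles far from the camera.
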(event `self.ReceiveBeginPlay`
  (bind _returnvalue (`KismetMaterialLibrary.CreateDynamicMaterialInstance` "/Game/Environment/Water/FluidInteractionTool/Blueprints/Data/M_FluidDraw.M_FluidDraw"))
  (set `self.FluidDrawMaterialInstanceDynamic` _returnvalue)
  (`NiagaraComponent.SetVariableObject` (`self.Rain`) "BPCallbackHandler" self)
  (`KismetSystemLibrary.K2_SetTimerDelegate` (`|CreateDelegate` :!event `Raining`) 0.5 true))

(event `self.ReceiveParticleData`
  (params (Data :type "Array of BasicParticleData Structure (by ref)") (NiagaraSystem :type "NiagaraSystem Object Reference") (SimulationPositionOffset :type "Vector Structure (by ref)"))
  (bind _returnvalue (`GameplayStatics.GetPlayerCameraManager` 0))
  (for _array_element Data
    (`/Engine/EditorBlueprintResources/StandardMacros.IsValid` (`self.FluidDrawMaterialInstanceDynamic`)
      (:`Is Valid`
        (`/Engine/EditorBlueprintResources/StandardMacros.IsValid` (`self.FluidControllerReference`)
          (:`Is Valid`
            (`/Engine/EditorBlueprintResources/StandardMacros.IsValid` _returnvalue
              (:`Is Valid`
                (bind _position (break `BasicParticleData` _array_element))
                (bind (_distance _outofradius) (`/Game/Environment/Water/FluidInteractionTool/Blueprints/BP_Fluid_FunctionLibrary.DistanceCheck` (`PlayerCameraManager.GetCameraLocation` _returnvalue) _position 4000.0))
                (if (not _outofradius)
                  (`/Game/Environment/Water/FluidInteractionTool/Blueprints/BP_Fluid_FunctionLibrary.DrawFluidSim` (`self.FluidControllerReference`) (`self.FluidDrawMaterialInstanceDynamic`) _position (`KismetMathLibrary.RandomFloatInRange` 0.0005 0.001) (`KismetMathLibrary.RandomFloatInRange` 0.1 0.2)))))))))))

(event `Raining`
  (`self.K2_SetActorLocation` (+ (`self.K2_GetActorLocation` (cast `/Game/GKnight/BP_PlayerCharacter` (`GameplayStatics.GetPlayerCharacter` 0) :!pure true)) (0.0 0.0 2500.0))))

(fn `UserConstructionScript`)