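; BP_Fireflies is an environmental firefly effect that shows only while the player has no detected enemies.
; A looping half-second timer started on BeginPlay checks the EnemiesDetected collection on the player's BP_PlayerCharacter.
; It activates the Niagara component without a reset when that collection is empty and deactivates it otherwise.
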(event `self.ReceiveBeginPlay`
  (`KismetSystemLibrary.K2_SetTimerDelegate` (delegate `SetFireflies`) 0.5 true))

(event `SetFireflies`
  (if (`KismetArrayLibrary.Array_IsEmpty` (`/Game/GKnight/BP_PlayerCharacter.EnemiesDetected` (cast `/Game/GKnight/BP_PlayerCharacter` (`GameplayStatics.GetPlayerCharacter` 0) :!pure true)))
    (`ActorComponent.Activate` (`self.Niagara`) false)
    (else
      (`ActorComponent.Deactivate` (`self.Niagara`)))))

(fn `UserConstructionScript`)