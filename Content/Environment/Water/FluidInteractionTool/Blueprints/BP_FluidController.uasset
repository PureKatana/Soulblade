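; BP_FluidController runs a GPU heightfield fluid simulation for interactive water in render targets.
; A fixed-rate accumulator on Tick, capped at 120 Hz, cycles three height targets, feeding the previous two frames into the simulation material to draw the next.
; After those steps, it writes the latest height and a computed normal map to the FluidOut and FluidOutNormal targets.
; Height targets and dynamic materials are created at BeginPlay.
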(event `self.ReceiveBeginPlay`
  ;[0 1 0] BeginPlay & EndPlay
  ;;[1 1 1] Clear Render Targets and Create Materials
  (`self.ClearRenderTargets`)
  (`self.CreateMaterials`))

(event `self.ReceiveEndPlay`
  (params (EndPlayReason :type "EEndPlayReason Enum" :default "Destroyed"))
  ;[0 1 0] BeginPlay & EndPlay
  ;;[1 1 1] Clear Render Targets on endplay
  (`self.ClearRenderTargets`))

(event `self.ReceiveTick`
  (params (DeltaSeconds :type "Float (single-precision)"))
  (bind _height_1 (`self.Height_1`))
  (bind _fluidsimulation (`self.FluidSimulation`))
  (bind _height_0 (`self.Height_0`))
  (bind _height_2 (`self.Height_2`))
  (bind _normalsimulation (`self.NormalSimulation`))
  (bind _fluidtransfer (`self.FluidTransfer`))
  ;[0 1 1] Tick
  (if (`self.EnableSimulation`)
    (`self.FluidUpdate` DeltaSeconds ; Fluid Sim While Loop
      (:`Fluid Sim Loop`
        ;;[1 1 1] Propagate the fluid sim with RT height frames
        (set `self.CurrentRT` (mod (+ (`self.CurrentRT`) 1) 3)) ; Cycle Current Height
        (bind _rendertargetout (`self.GetPreviousRT` (`self.CurrentRT`) 1 _height_0 _height_1 _height_2))
        (`MaterialInstanceDynamic.SetTextureParameterValue` _fluidsimulation "PreviousHeight_1" _rendertargetout)
        (bind _rendertargetout_2 (`self.GetPreviousRT` (`self.CurrentRT`) 2 _height_0 _height_1 _height_2))
        (`MaterialInstanceDynamic.SetTextureParameterValue` _fluidsimulation "PreviousHeight_2" _rendertargetout_2)
        (bind _rendertarget (`self.GetRT` (`self.CurrentRT`) _height_0 _height_1 _height_2))
        (bind (_canvas _size _context) (`KismetRenderingLibrary.BeginDrawCanvasToRenderTarget` _rendertarget))
        (`Canvas.K2_DrawMaterial` _canvas _fluidsimulation (0.0 0.0) _size (0.0 0.0) (1.0 1.0) 0.0 (0.5 0.5))
        (`KismetRenderingLibrary.EndDrawCanvasToRenderTarget` _context))
      (:`Completed`
        ;;[1 1 1] On completion of the fluid sim transfer the render target height to the completed RT and Compute the normal
        (bind _rendertarget_2 (`self.GetRT` (`self.CurrentRT`) (`self.Height_0`) (`self.Height_1`) (`self.Height_2`)))
        (`MaterialInstanceDynamic.SetTextureParameterValue` _normalsimulation "PreviousHeight_1" _rendertarget_2)
        (`KismetRenderingLibrary.DrawMaterialToRenderTarget` (`self.FluidOutNormal`) _normalsimulation)
        (`MaterialInstanceDynamic.SetTextureParameterValue` _fluidtransfer "Fluid" _rendertarget_2)
        (`KismetRenderingLibrary.DrawMaterialToRenderTarget` (`self.FluidOut`) _fluidtransfer)))))

(fn `ClearRenderTargets`
  ;[1 1 1] Clear all render targets
  (`KismetRenderingLibrary.ClearRenderTarget2D` (`self.Height_0`))
  (`KismetRenderingLibrary.ClearRenderTarget2D` (`self.Height_1`))
  (`KismetRenderingLibrary.ClearRenderTarget2D` (`self.Height_2`))
  (`KismetRenderingLibrary.ClearRenderTarget2D` (`self.FluidOut`))
  (`KismetRenderingLibrary.ClearRenderTarget2D` (`self.FluidOutNormal`) (struct :`B` 1.0 :`A` 1.0)))

(fn `CreateMaterials`
  (bind _rendertargetsize (`self.RenderTargetSize`))
  ;[0 1 0] Create Materials
  (`|ExecutionSequence`
    (:`then_0`
      ;;[1 1 1] Setup fluid sim render targets
      (bind _returnvalue (`KismetRenderingLibrary.CreateRenderTarget2D` _rendertargetsize _rendertargetsize))
      (set `self.Height_0` _returnvalue)
      (bind _returnvalue_2 (`KismetRenderingLibrary.CreateRenderTarget2D` _rendertargetsize _rendertargetsize))
      (set `self.Height_1` _returnvalue_2)
      (bind _returnvalue_3 (`KismetRenderingLibrary.CreateRenderTarget2D` _rendertargetsize _rendertargetsize))
      (set `self.Height_2` _returnvalue_3))
    (:`then_1`
      ;;[1 1 1] Create Fluid sim dynamic material instances
      (bind _returnvalue_4 (`KismetMaterialLibrary.CreateDynamicMaterialInstance` "/Game/Environment/Water/FluidInteractionTool/Blueprints/Data/M_FluidTransfer.M_FluidTransfer"))
      (set `self.FluidTransfer` _returnvalue_4)
      (bind _returnvalue_5 (`KismetMaterialLibrary.CreateDynamicMaterialInstance` "/Game/Environment/Water/FluidInteractionTool/Blueprints/Data/M_NormalCalculation.M_NormalCalculation"))
      (bind _output_get (set `self.NormalSimulation` _returnvalue_5))
      (bind _returnvalue_6 (`KismetMaterialLibrary.CreateDynamicMaterialInstance` "/Game/Environment/Water/FluidInteractionTool/Blueprints/Data/M_HeightSimulator.M_HeightSimulator"))
      (bind _output_get_2 (set `self.FluidSimulation` _returnvalue_6))
      ;;[1 1 1] Set Height Simulation Fampening and Travel Speed
      (`MaterialInstanceDynamic.SetScalarParameterValue` _output_get_2 "FluidDampening" (`self.FluidDampening`))
      (`MaterialInstanceDynamic.SetScalarParameterValue` _output_get_2 "FluidTravelSpeed" (`self.FluidTravelSpeed`))
      (`MaterialInstanceDynamic.SetScalarParameterValue` _output_get "Intensity" (`self.NormalIntensity`)) ; Set normal intensity
    )))

(fn `GetPreviousRT`
  (params (CurrentRTIndex :type Integer) (FramesOld :type Integer) (RenderTarget_0 :type "TextureRenderTarget2D Object Reference") (RenderTarget_1 :type "TextureRenderTarget2D Object Reference") (RenderTarget_2 :type "TextureRenderTarget2D Object Reference"))
  (returns (RenderTargetOut :type "TextureRenderTarget2D Object Reference"))
  ;[1 1 1] Get Previous Height RT
  (bind _rendertarget (`self.GetRT` (mod (+ (- CurrentRTIndex FramesOld) 3) 3) RenderTarget_0 RenderTarget_1 RenderTarget_2))
  (return _rendertarget))

(fn `GetRT`
  (params (Index :type Integer) (RenderTarget_0 :type "TextureRenderTarget2D Object Reference") (RenderTarget_1 :type "TextureRenderTarget2D Object Reference") (RenderTarget_2 :type "TextureRenderTarget2D Object Reference"))
  (returns (RenderTarget :type "TextureRenderTarget2D Object Reference"))
  ;[1 1 1] Get render target via Index
  (return (select `int` Index :`0` RenderTarget_0 :`1` RenderTarget_1 :`2` RenderTarget_2)))

(fn `GetRT_Height`
  (params (Index :type Integer))
  (returns (RenderTarget :type "TextureRenderTarget2D Object Reference"))
  ;[1 1 1] Get render target via Index
  (return (select `int` Index :`0` (`self.Height_0`) :`1` (`self.Height_1`) :`2` (`self.Height_2`))))

(fn `UserConstructionScript`
  (`self.ClearRenderTargets`))