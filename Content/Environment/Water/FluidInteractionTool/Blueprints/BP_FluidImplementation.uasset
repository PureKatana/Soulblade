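; Component that lets its owning actor disturb a fluid simulation on tagged water surfaces.
; On BeginPlay it finds BP_FluidController by tag and creates a dynamic draw material.
; Each tick, after distance and optional visibility culling, it line-traces at the actor or mesh bones and draws into the sim on hits.
; Velocity can gate drawing and scale single-point intensity, while per-bone intensity stays at maximum.
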(event `self.ReceiveBeginPlay`
  (bind _returnvalue (`self.GetOwner`))
  ;[0 1 0] Begin Play
  (`|ExecutionSequence`
    (:`then_0`
      ;;[1 1 1] Find Controller
      (`/Engine/EditorBlueprintResources/StandardMacros.IsValid` (`self.FluidControllerReference`)
        (:`Is Valid`
          _)
        (:`Is Not Valid`
          (`self.FindFluidController`)))
      ;;[1 1 1] Get Mesh Components For Per Bone Trace
      (if (`self.UsePerBoneTrace`)
        (`/Engine/EditorBlueprintResources/StandardMacros.IsValid` _returnvalue
          (:`Is Valid`
            (set `self.MeshComponents` (`Actor.GetComponentsByTag` _returnvalue "/Script/Engine.MeshComponent" (`self.FluidMeshTag`)))))))
    (:`then_1`
      (bind _returnvalue_2 (`KismetMaterialLibrary.CreateDynamicMaterialInstance` "/Game/Environment/Water/FluidInteractionTool/Blueprints/Data/M_FluidDraw.M_FluidDraw"))
      (set `self.DrawMaterialInstanceDynamic` _returnvalue_2))))

(event `self.ReceiveTick`
  (params (DeltaSeconds :type "Float (single-precision)"))
  (bind _returnvalue (`self.GetOwner`))
  (bind _returnvalue_2 (`GameplayStatics.GetPlayerCameraManager` 0))
  (bind _returnvalue_3 (`Actor.K2_GetActorLocation` _returnvalue))
  (bind _returnvalue_4 (`KismetMathLibrary.Abs` (`KismetMathLibrary.VSize` (`Actor.GetVelocity` _returnvalue))))
  ;[0 1 1] Tick
  (`/Engine/EditorBlueprintResources/StandardMacros.IsValid` (`self.FluidControllerReference`) ; Check if Fluid Controller is Valid
    (:`Is Valid`
      (if (`self.UseFrustumCulling`)
        ;;[1 1 1] Distance Check from player camera
        (if (`Actor.WasRecentlyRendered` _returnvalue 0.1)
          (`/Engine/EditorBlueprintResources/StandardMacros.IsValid` _returnvalue_2 :!label _label
            (:`Is Valid`
              (bind (_distance _outofradius) (`/Game/Environment/Water/FluidInteractionTool/Blueprints/BP_Fluid_FunctionLibrary.DistanceCheck` (`Actor.K2_GetActorLocation` _returnvalue_2) _returnvalue_3 (`self.FluidCullDistance`)))
              (if (not _outofradius)
                (if (`self.UsePerBoneTrace`)
                  ;;[1 1 1] Per Bone Trace And Draw
                  (for _array_element (`self.MeshComponents`)
                    (`/Engine/EditorBlueprintResources/StandardMacros.IsValid` _array_element
                      (:`Is Valid`
                        (if (<= (`KismetArrayLibrary.Array_Length` (`self.Bones to Ignore`)) 0)
                          (bind _returnvalue_5 (`SceneComponent.GetAllSocketNames` _array_element))
                          (for _array_element_2 _returnvalue_5
                            (`self.PerBoneDraw` _array_element_2 _array_element))
                          (else
                            (for _array_element_3 _returnvalue_5
                              (if (not (`KismetArrayLibrary.Array_Contains` (`self.Bones to Ignore`) _array_element_3))
                                (`self.PerBoneDraw` _array_element_3 _array_element))))))))
                  (else
                    ;;[1 1 1] Single Fluid Trace And Draw
                    (if (`self.VelocityDeterminesIntensity`)
                      (if (> _returnvalue_4 (`self.VelocityBegin`))
                        (bind _valid (`self.FluidTrace` _returnvalue_3 :!label _label_2))
                        (if _valid
                          (`/Game/Environment/Water/FluidInteractionTool/Blueprints/BP_Fluid_FunctionLibrary.DrawFluidSim` (`self.FluidControllerReference`) (`self.DrawMaterialInstanceDynamic`) _returnvalue_3 (`self.FluidDrawSize`) (* (select `bool` (`self.VelocityDeterminesIntensity`) :`false` 1.0 :`true` (/ _returnvalue_4 (`self.VelocityDivideIntensity`))) (`self.FluidMaxDrawIntensity`)))))
                      (else
                        (goto _label_2)))))))))
        (else
          (goto _label))))))

(fn `FindFluidController`
  ;[1 1 1] Get all actors with tag and cast to the fluid controller, break on first
  (bind _outactors (`GameplayStatics.GetAllActorsWithTag` (`self.FluidControllerTag`)))
  (if (> (`KismetArrayLibrary.Array_Length` _outactors) 0)
    (for _array_element _outactors
      (`/Engine/EditorBlueprintResources/StandardMacros.IsValid` _array_element
        (:`Is Valid`
          (bind _asbp_fluid_controller (cast `/Game/Environment/Water/FluidInteractionTool/Blueprints/BP_FluidController` _array_element))
          (set `self.FluidControllerReference` _asbp_fluid_controller)
          (break))))
    (else
      (`KismetSystemLibrary.PrintString` "No Fluid Controller Found!" true true (struct :`R` 1.0 :`A` 1.0)) ; Return false with warning message
    )))

(fn `FluidTrace`
  (params (Location :type "Vector Structure"))
  (returns (Valid :type Boolean))
  (bind _fluidsurfacetag (`self.FluidSurfaceTag`))
  ;[1 1 1] Line trace by channel to find water surface by tag
  (bind (_outhit _returnvalue) (`KismetSystemLibrary.LineTraceSingle` :`Start` (+ Location (`KismetMathLibrary.MakeVector` 0.0 0.0 (`self.TraceOffsetUp`))) :`End` (+ Location (`KismetMathLibrary.MakeVector` 0.0 0.0 (`self.TraceOffsetDown`))) :`TraceChannel` "TraceTypeQuery1" :`DrawDebugType` (select `bool` (`self.ShowTraceDebug`) :`true` "ForDuration" :!type "EDrawDebugTrace Enum") :`DrawTime` 1.0))
  (bind (_bblockinghit _binitialoverlap _time _distance _location _impactpoint _normal _impactnormal _physmat _hitactor _hitcomponent) (`GameplayStatics.BreakHitResult` _outhit))
  (if (and _returnvalue _bblockinghit)
    (if (or (`Actor.ActorHasTag` _hitactor _fluidsurfacetag) (`self.ComponentHasTag` _hitcomponent _fluidsurfacetag))
      (return true)
      (else
        _)))
  (return false) ; Return false if no fluid surface found
)

(fn `PerBoneDraw`
  (params (`Bone Name` :type Name) (`Mesh Component` :type "MeshComponent Object Reference (by ref)"))
  (bind _returnvalue (`SceneComponent.GetSocketLocation` `Mesh Component` `Bone Name`))
  ;[1 1 1] Trace and draw via bone/socket location with velocity checks
  (bind _returnvalue_2 (`PrimitiveComponent.GetPhysicsLinearVelocity` `Mesh Component` `Bone Name`))
  (if (`self.VelocityDeterminesIntensity`)
    (bind _returnvalue_3 (`KismetMathLibrary.Abs` (`KismetMathLibrary.VSize` _returnvalue_2)))
    (if (> _returnvalue_3 (`self.VelocityBegin`))
      (bind _valid (`self.FluidTrace` _returnvalue :!label _label))
      (if _valid
        (`/Game/Environment/Water/FluidInteractionTool/Blueprints/BP_Fluid_FunctionLibrary.DrawFluidSim` (`self.FluidControllerReference`) (`self.DrawMaterialInstanceDynamic`) _returnvalue (`self.FluidDrawSize`) (* (select `bool` false :`false` 1.0 :`true` (/ _returnvalue_3 (`self.VelocityDivideIntensity`))) (`self.FluidMaxDrawIntensity`)))))
    (else
      (goto _label))))