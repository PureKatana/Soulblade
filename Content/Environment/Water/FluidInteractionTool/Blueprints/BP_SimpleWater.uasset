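; BP_SimpleWater is a water actor that builds an ocean plane from a square grid of tiled meshes.
; GenerateOceanPlane clears a Hierarchical Instanced Static Mesh component, assigns the water mesh and material, then adds instances in a nested loop.
; Tile spacing derives from the mesh bounds and a horizontal scale multiplier, assuming a centered pivot.
; The event graph and construction script are empty, so generation runs only when that function is invoked.
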(fn `GenerateOceanPlane`
  (bind _waterplanemesh (`self.WaterPlaneMesh`))
  (bind _hierarchicalinstancedstaticmesh (`self.HierarchicalInstancedStaticMesh`))
  (bind _tilecount (`self.TileCount`))
  (bind _watermaterial (`self.WaterMaterial`))
  (bind _meshscaleoffset (`self.MeshScaleOffset`))
  (bind (_returnvalue_min _returnvalue_max) (break `Box` (`StaticMesh.GetBoundingBox` _waterplanemesh)))
  (bind (_returnvalue_x _returnvalue_y) (`KismetMathLibrary.BreakVector` (* (* _returnvalue_max (`self.MeshScaleOffset`)) 2.0)))
  ;[1 1 1] Clear instances first
  (`InstancedStaticMeshComponent.ClearInstances` (`self.HierarchicalInstancedStaticMesh`))
  ;[1 1 1] Set Mesh and Material on Instance Component
  (`/Engine/EditorBlueprintResources/StandardMacros.IsValid` _waterplanemesh
    (:`Is Valid`
      (`StaticMeshComponent.SetStaticMesh` _hierarchicalinstancedstaticmesh _waterplanemesh)
      (`/Engine/EditorBlueprintResources/StandardMacros.IsValid` _watermaterial
        (:`Is Valid`
          (`PrimitiveComponent.SetMaterial` _hierarchicalinstancedstaticmesh 0 _watermaterial)
          ;[1 1 1] 2d array loop
          (for _index (range (+ _tilecount 1))
            (for _index_2 (range (+ _tilecount 1))
              ;[1 1 1] Add instance
              (`InstancedStaticMeshComponent.AddInstance` (`self.HierarchicalInstancedStaticMesh`) (`KismetMathLibrary.MakeTransform` (`KismetMathLibrary.MakeVector` (* _index _returnvalue_x) (* _index_2 _returnvalue_y)) (struct) (`KismetMathLibrary.MakeVector` _meshscaleoffset _meshscaleoffset 1.0)) false))))))))

(fn `UserConstructionScript`)