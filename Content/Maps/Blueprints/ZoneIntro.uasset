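; ZoneIntro is a placeable trigger volume that announces a named zone and switches its music when the player enters.
; On box overlap by BP_PlayerCharacter, it gets player 0's BP_PlayerController and, if CurrentZone differs from ZoneText, sets the zone text and replaces any current music with ZoneMusic.
; CurrentZone updates only on end overlap, through the cached controller, without checking which actor left.
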(event `self.Box.OnComponentBeginOverlap`
  (params (OverlappedComponent :type "PrimitiveComponent Object Reference") (OtherActor :type "Actor Object Reference") (OtherComp :type "PrimitiveComponent Object Reference") (OtherBodyIndex :type Integer) (bFromSweep :type Boolean) (SweepResult :type "HitResult Structure (by ref)"))
  (bind _playercontroller (`self.PlayerController`))
  (cast `/Game/GKnight/BP_PlayerCharacter` OtherActor)
  (bind _asbp_player_controller (cast `/Game/GKnight/BP_PlayerController` (`GameplayStatics.GetPlayerController` 0)))
  (bind _output_get (set `self.PlayerController` _asbp_player_controller))
  (if (!= (`/Game/GKnight/BP_PlayerController.CurrentZone` _output_get) (`self.ZoneText`))
    (`/Game/GKnight/BP_PlayerController.SetZoneText` _output_get (`self.ZoneText`))
    (`/Engine/EditorBlueprintResources/StandardMacros.IsValid` (`/Game/GKnight/BP_PlayerController.GetMusic` (`self.PlayerController`))
      (:`Is Valid`
        (`/Game/GKnight/BP_PlayerController.StopMusic` (`self.PlayerController`)))
      (:`Is Not Valid`
        _))
    (`/Game/GKnight/BP_PlayerController.SetMusic` _playercontroller (`self.ZoneMusic`))
    (`/Game/GKnight/BP_PlayerController.PlayMusic` _playercontroller)))

(event `self.Box.OnComponentEndOverlap`
  (params (OverlappedComponent :type "PrimitiveComponent Object Reference") (OtherActor :type "Actor Object Reference") (OtherComp :type "PrimitiveComponent Object Reference") (OtherBodyIndex :type Integer))
  (bind _playercontroller (`self.PlayerController`)
    (:`then`
      (set `/Game/GKnight/BP_PlayerController.CurrentZone` (`self.ZoneText`) _playercontroller))
    (:`else`)))

(fn `UserConstructionScript`)