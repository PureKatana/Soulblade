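; Main menu player character that shows the menu widget and displays a weapon-equip animation.
; After a delay on BeginPlay it creates W_MainMenu and binds the widget's EquipWeapon dispatcher to play the Protector equip montage.
; A separate EquipWeapon event, not called within this Blueprint, attaches sword and shield to mesh sockets and sends the anim instance a combat type update.
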(event `self.ReceiveBeginPlay`
  (`KismetSystemLibrary.Delay` 5.0)
  (bind _returnvalue (`|CreateWidget` "/Game/UI/W_MainMenu.W_MainMenu_C"))
  (`UserWidget.AddToViewport` _returnvalue 0)
  (add `/Game/UI/W_MainMenu.EquipWeapon` _returnvalue (delegate `PlayAnim`)))

(event `PlayAnim`
  (`|PlayMontage` (`self.SkeletalMesh`) "/Game/GKnight/Animation/SwordAndShield/Protector_Equip_Montage1.Protector_Equip_Montage1"))

(event `EquipWeapon`
  (`SceneComponent.K2_AttachToComponent` (`self.Sword`) (`self.SkeletalMesh`) "WeaponSocket" "KeepRelative" "KeepRelative" "KeepRelative" true)
  (`SceneComponent.K2_AttachToComponent` (`self.Shield`) (`self.SkeletalMesh`) "ShieldSocket" "KeepRelative" "KeepRelative" "KeepRelative" true)
  (message `/Game/CombatSystem/Blueprints/Interfaces/AnimInstance_BPI.UpdateCombatType` (`SkeletalMeshComponent.GetAnimInstance` (`self.SkeletalMesh`)) "NewEnumerator1"))

(fn `UserConstructionScript`)