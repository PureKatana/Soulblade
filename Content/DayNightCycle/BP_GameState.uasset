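; BP_GameState runs the game's day-night clock by driving the time of day on the level's BP_SunSky actor.
; On BeginPlay it finds that actor, converts its starting time into total seconds and starts a looping timer at a configurable tick rate.
; Each tick adds a set number of seconds, writes hours, minutes and seconds back to the sky, then resets the counter after a full day.
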(event `self.ReceiveBeginPlay`
  (bind _returnvalue (`GameplayStatics.GetActorOfClass` "/Game/DayNightCycle/BP_SunSky.BP_SunSky_C"))
  (bind _output_get (set `self.SunSky` _returnvalue))
  (set `self.TimeOfDayInSeconds` (`KismetMathLibrary.FTrunc` (`KismetMathLibrary.GetTotalSeconds` (`KismetMathLibrary.MakeTimespan` 0 (`/Game/DayNightCycle/BP_SunSky.Hours` _output_get) (`/Game/DayNightCycle/BP_SunSky.Minutes` _output_get) (`/Game/DayNightCycle/BP_SunSky.Seconds` _output_get)))))
  (`KismetSystemLibrary.K2_SetTimerDelegate` (delegate `TimeUpdate`) (/ 1.0 (`self.AmountToTickASecond`)) true))

(event `TimeUpdate`
  (bind _sunsky (`self.SunSky`))
  (bind _output_get (set `self.TimeOfDayInSeconds` (+ (`self.TimeOfDayInSeconds`) (`self.AmountOfSecondsToAddPerTick`))))
  (bind (_days _hours _minutes _seconds) (`KismetMathLibrary.BreakTimespan` (`KismetMathLibrary.MakeTimespan` 0 0 0 _output_get)))
  (set `/Game/DayNightCycle/BP_SunSky.Hours` _hours _sunsky)
  (set `/Game/DayNightCycle/BP_SunSky.Minutes` _minutes _sunsky)
  (set `/Game/DayNightCycle/BP_SunSky.Seconds` _seconds _sunsky)
  (if (>= (`self.TimeOfDayInSeconds`) 86400)
    (set `self.TimeOfDayInSeconds` 0)))

(fn `UserConstructionScript`)